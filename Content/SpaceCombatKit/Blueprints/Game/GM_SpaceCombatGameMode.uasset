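; Space combat game mode that handles faction assignment, player respawns and supplying fighter pilots from capital ships.
; Players get a faction mothership, view it during a delay, then join a queue for its available fighters, with default-pawn respawn as fallback.
; Each queue pass, also timed after team-select starts, then gives leftover fighters AI controllers, launching 6DoF ones from hangars.
; Camera transitions use blends, or fades with an HMD.
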(event `RespawnPlayer`
  (params (Controller :type "PlayerController Object Reference"))
  ;[1 1 1] Respawn player - wait 3 seconds, add their controller to controllers waiting for fighter. Blend their view to their capital while they wait.. Then call get a fighter for them.
  (bind _aspc_space_combat_controller (cast `/Game/SpaceCombatKit/Blueprints/Game/PC_SpaceCombatController` Controller)
    (:`then`
      (bind _mothercapitalship (`/Game/SpaceCombatKit/Blueprints/Game/PC_SpaceCombatController.MotherCapitalShip` _aspc_space_combat_controller))
      (`/Engine/EditorBlueprintResources/StandardMacros.IsValid` _mothercapitalship ; Makes sure they have a parent capital
        (:`Is Valid`
          ;;[1 1 1] Spawns a default pawn so we can set view target with blend
          (bind _returnvalue (`|SpawnActorFromClass` "/Script/Engine.DefaultPawn" (`KismetMathLibrary.MakeTransform` (`self.K2_GetActorLocation` _mothercapitalship)) "Undefined" "OverrideRootScale" null null))
          (`Controller.Possess` _aspc_space_combat_controller _returnvalue)
          (`self.CameraTransition` _aspc_space_combat_controller _mothercapitalship 2.0 2.0)
          (`KismetSystemLibrary.Delay` 3.0)
          (`KismetArrayLibrary.Array_Add` (`self.ControllersWaitingForFighter`) _aspc_space_combat_controller)
          (`self.GetFightersForControllers`))
        (:`Is Not Valid`
          (`self.RespawnAsDefaultClass` Controller :!label _label) ; Respawns the player as a default class
        )))
    (:`CastFailed`
      (goto _label))))

(event `AssignFactionToPC`
  (params (FactionToAssign :type "/Game/SpaceCombatKit/Blueprints/Game/E_FactionsEnum Enum" :default "NewEnumerator0") (Controller :type "PlayerController Object Reference"))
  ;[1 1 1] Assigns a faction to a PC - also assigns a mothership based on that faction, and looks at it.
  (bind _aspc_space_combat_controller (cast `/Game/SpaceCombatKit/Blueprints/Game/PC_SpaceCombatController` Controller)
    (:`then`
      (bind _output_get (set `/Game/SpaceCombatKit/Blueprints/Game/PC_SpaceCombatController.Faction` FactionToAssign _aspc_space_combat_controller))
      (bind _output_get_2 (set `/Game/SpaceCombatKit/Blueprints/Game/PC_SpaceCombatController.MotherCapitalShip` (`self.GetAvailableCapitalShip` _output_get) _aspc_space_combat_controller))
      (`self.CameraTransition` _aspc_space_combat_controller _output_get_2 2.0 2.0)
      (bind _aspawn_starting_team_select (cast `/Game/SpaceCombatKit/Blueprints/Game/Pawn_StartingTeamSelect` (`Controller.K2_GetPawn` _aspc_space_combat_controller)))
      (`/Game/SpaceCombatKit/Blueprints/Game/Pawn_StartingTeamSelect.RemoveWidgets` _aspawn_starting_team_select null))
    (:`CastFailed`
      _))
  (`KismetSystemLibrary.Delay` 3.0)
  (`KismetArrayLibrary.Array_Add` (`self.ControllersWaitingForFighter`) _aspc_space_combat_controller)
  (`self.GetFightersForControllers`))

(event `self.ReceiveBeginPlay`
  ;[1 1 1] Begin play - set a timer that checks every 5 seconds if there's any controllers waiting for a fighter - but only if their starting pawn was a team select pawn
  (if (== (`GameplayStatics.GetPlayerPawn` 0) "/Game/SpaceCombatKit/Blueprints/Game/Pawn_StartingTeamSelect.Pawn_StartingTeamSelect")
    (`KismetSystemLibrary.K2_SetTimerDelegate` (delegate `GetFightersForControllers`) 5.0 true)))

(event `GetFightersForControllers`
  (bind _controllerswaitingforfighter (`self.ControllersWaitingForFighter`))
  ;[1 1 1] Get fighter for controllers - check the controllers mothership, and assign it a fighter from there
  (for _array_element _controllerswaitingforfighter
    (bind _mothercapitalship (`/Game/SpaceCombatKit/Blueprints/Game/PC_SpaceCombatController.MotherCapitalShip` _array_element))
    (if (`KismetArrayLibrary.Array_IsValidIndex` (`/Game/SpaceCombatKit/Blueprints/Ships/BaseClasses/BaseCapital.AvailableFighters` _mothercapitalship))
      (`/Game/SpaceCombatKit/Blueprints/Ships/BaseClasses/BaseCapital.AssignFighter` _mothercapitalship _array_element)
      (if (`HeadMountedDisplayFunctionLibrary.IsHeadMountedDisplayEnabled`)
        (`PlayerCameraManager.StartCameraFade` :`self` (`PlayerController.PlayerCameraManager` _array_element) :`FromAlpha` 1.0 :`Duration` 1.0 :`bHoldWhenFinished` true))
      (`KismetArrayLibrary.Array_RemoveItem` _controllerswaitingforfighter _array_element)))
  ;;[1 1 1] If no Player Controllers in waiting, spawn an AI controller, possess a fighter, and tell it to leave the hanger
  (bind _outactors (`GameplayStatics.GetAllActorsOfClass` "/Game/SpaceCombatKit/Blueprints/Ships/BaseClasses/BaseCapital.BaseCapital_C"))
  (for _array_element_2 _outactors
    (bind (_arrayindex _arrayelement) (`/Engine/EditorBlueprintResources/StandardMacros.ReverseForEachLoop` (`/Game/SpaceCombatKit/Blueprints/Ships/BaseClasses/BaseCapital.AvailableFighters` _array_element_2))
      (:`LoopBody`
        (bind _returnvalue (`|SpawnActorFromClass` (`Pawn.AIControllerClass` _arrayelement) (`KismetMathLibrary.MakeTransform` (0.0 0.0 0.0)) "Undefined" "OverrideRootScale" null null))
        (`/Game/SpaceCombatKit/Blueprints/Ships/BaseClasses/BaseCapital.AssignFighter` _array_element_2 _returnvalue)
        ;[1 1 1] If the fighter is a 6dof ai, tell it to launch from hangar
        (bind _asaicon_6do_ffighter_ai (cast `/Game/SpaceCombatKit/Blueprints/AI/AICon_6DoFFighterAI` _returnvalue))
        (`/Game/SpaceCombatKit/Blueprints/AI/AICon_6DoFFighterAI.LaunchFromhangar` _asaicon_6do_ffighter_ai)))))

(fn `CameraTransition`
  (params (Target :type "PlayerController Object Reference") (NewViewTarget :type "Actor Object Reference") (BlendTime :type "Float (double-precision)") (BlendExp :type "Float (double-precision)"))
  (if (`HeadMountedDisplayFunctionLibrary.IsHeadMountedDisplayEnabled`)
    (`PlayerCameraManager.StartCameraFade` :`self` (`PlayerController.PlayerCameraManager` Target) :`ToAlpha` 1.0 :`Duration` BlendTime :`bHoldWhenFinished` true)
    (else
      (`PlayerController.SetViewTargetWithBlend` Target NewViewTarget BlendTime "VTBlend_EaseInOut" BlendExp true))))

(fn `GetAvailableCapitalShip`
  (params (Faction :type "/Game/SpaceCombatKit/Blueprints/Game/E_FactionsEnum Enum" :default "NewEnumerator0"))
  (returns (CapitalShip :type "/Game/SpaceCombatKit/Blueprints/Ships/BaseClasses/BaseCapital Object Reference"))
  (locals (TempCapShip :type "/Game/SpaceCombatKit/Blueprints/Ships/BaseClasses/BaseCapital Object Reference"))
  (bind _tempcapship (`local.TempCapShip`))
  (bind _outactors (`GameplayStatics.GetAllActorsOfClass` "/Game/SpaceCombatKit/Blueprints/Ships/BaseClasses/BaseCapital.BaseCapital_C"))
  (for _array_element _outactors
    (if (`|EnumEquality` (`/Game/SpaceCombatKit/Blueprints/Ships/BaseClasses/BaseShip.Faction` _array_element) Faction)
      (set `local.TempCapShip` _array_element)
      (break)))
  (`/Engine/EditorBlueprintResources/StandardMacros.IsValid` _tempcapship
    (:`Is Valid`
      (return _tempcapship))
    (:`Is Not Valid`
      (`KismetSystemLibrary.PrintString` "No Available Motherships!"))))

(fn `RespawnAsDefaultClass`
  (params (Controller :type "PlayerController Object Reference"))
  ;[1 1 1] Spawns a default pawn from the game mode and possesses it for the given controller
  (bind _outactors (`GameplayStatics.GetAllActorsOfClass` "/Script/Engine.PlayerStart"))
  (bind _returnvalue (`|SpawnActorFromClass` (`GameModeBase.DefaultPawnClass` (`GameplayStatics.GetGameMode`)) (`self.GetTransform` (`|GetArrayItem` _outactors)) "AdjustIfPossibleButAlwaysSpawn" "OverrideRootScale" null null))
  (`Controller.Possess` Controller _returnvalue))

(fn `UserConstructionScript`)