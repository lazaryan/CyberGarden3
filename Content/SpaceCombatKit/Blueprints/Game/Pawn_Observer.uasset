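; Free-flying observer pawn that films ships with a cine camera, with boost and smoothed focal-length zoom.
; Hotkeys pick a ship to track: nearest, random, or a FireLance capital ship by faction.
; Tick rotates the camera toward the ship's position plus velocity and focuses at its distance.
; The pawn can also glide to the ship's cycled camera components, optionally offset in front, at adjustable speed; SetBlendView is never called.
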(event `Key|MouseScrollDown`
  (params (Key :type "Key Structure" :default "AnyKey"))
  (bind _minfocal (`self.MinFocal`))
  (bind _zoomspeed (`self.ZoomSpeed`))
  (bind _maxfocal (`self.MaxFocal`))
  ;[1 1 1] Zooming
  (:`Pressed`
    (set `self.DefaultFocal` (`KismetMathLibrary.FClamp` (- (`self.DefaultFocal`) _zoomspeed) _minfocal _maxfocal))
    (set `self.TargetFocal` (`KismetMathLibrary.FClamp` (- (`self.TargetFocal`) _zoomspeed) _minfocal _maxfocal))))

(event `Key|MouseScrollUp`
  (params (Key :type "Key Structure" :default "AnyKey"))
  (bind _minfocal (`self.MinFocal`))
  (bind _zoomspeed (`self.ZoomSpeed`))
  (bind _maxfocal (`self.MaxFocal`))
  ;[1 1 1] Zooming
  (:`Pressed`
    (set `self.DefaultFocal` (`KismetMathLibrary.FClamp` (+ (`self.DefaultFocal`) _zoomspeed) _minfocal _maxfocal))
    (set `self.TargetFocal` (`KismetMathLibrary.FClamp` (+ (`self.TargetFocal`) _zoomspeed) _minfocal _maxfocal))))

(event `InputAxis|MoveForward`
  (params (AxisValue :type "Float (single-precision)"))
  ;[1 1 1] Movement
  (`PawnMovementComponent.AddInputVector` (`self.FloatingPawnMovement`) (* (`self.GetActorRightVector`) (stale `InputAxis|MoveRight` AxisValue)) false))

(event `self.ReceiveBeginPlay`
  ;[1 1 1] Begin play, set default max speed to use for boosting
  (set `self.DefaultMaxSpeed` (`MovementComponent.GetMaxSpeed` (`self.FloatingPawnMovement`)))
  (bind _output_get (set `self.DefaultFocal` (`CineCameraComponent.CurrentFocalLength` (`self.CineCamera`))))
  (set `self.TargetFocal` _output_get))

(event `InputAxis|MoveRight`
  (params (AxisValue :type "Float (single-precision)"))
  ;[1 1 1] Movement
  (`PawnMovementComponent.AddInputVector` (`self.FloatingPawnMovement`) (* (`self.GetActorForwardVector`) (stale `InputAxis|MoveForward` AxisValue)) false))

(event `InputAxis|LookUp`
  (params (AxisValue :type "Float (single-precision)"))
  ;[1 1 1] Turning
  (`self.K2_AddActorLocalRotation` (`KismetMathLibrary.MakeRotator` 0.0 AxisValue)))

(event `Key|Three`
  (params (Key :type "Key Structure" :default "AnyKey"))
  ;[1 1 1] Get and track random ship
  (:`Pressed`
    (bind _randomship (`self.GetRandomShip`))
    (set `self.ShipToTrack` _randomship)))

(event `InputAction|AltFire`
  (params (Key :type "Key Structure" :default "AnyKey"))
  (bind _defaultfocal (`self.DefaultFocal`))
  ;[1 1 1] Zoom in
  (:`Pressed`
    (set `self.TargetFocal` (/ _defaultfocal 0.6)))
  (:`Released`
    (set `self.TargetFocal` _defaultfocal)))

(event `InputAxis|TurnRight`
  (params (AxisValue :type "Float (single-precision)"))
  ;[1 1 1] Turning
  (`self.K2_AddActorLocalRotation` (`KismetMathLibrary.MakeRotator` 0.0 0.0 AxisValue)))

(event `Key|One`
  (params (Key :type "Key Structure" :default "AnyKey"))
  ;[1 1 1] Follow Capital Ships on 1/2 press
  (:`Pressed`
    (`/Engine/EditorBlueprintResources/StandardMacros.IsValid` (`self.ShipToBlendView`)
      (:`Is Valid`
        (`self.StopBlendView` :!label _label) ; Stops tracking a ship if we are tracking one
      )
      (:`Is Not Valid`
        (bind _outactors (`GameplayStatics.GetAllActorsOfClass` "/Game/SpaceCombatKit/Blueprints/Ships/SteeringShip_Capital_FireLance.SteeringShip_Capital_FireLance_C"))
        (for _array_element _outactors
          (if (`|EnumEquality` (`/Game/SpaceCombatKit/Blueprints/Ships/BaseClasses/BaseShip.Faction` _array_element) "NewEnumerator2")
            (set `self.ShipToBlendView` _array_element)
            (break)))
        (set `self.ShipToTrack` (`self.ShipToBlendView`) :!label _label_2)
        (set `self.ShipToBlendView` null)))))

(event `Key|LeftShift`
  (params (Key :type "Key Structure" :default "AnyKey"))
  (bind _floatingpawnmovement (`self.FloatingPawnMovement`))
  (bind _defaultmaxspeed (`self.DefaultMaxSpeed`))
  ;[1 1 1] Boost
  (:`Pressed`
    (set `FloatingPawnMovement.MaxSpeed` (* _defaultmaxspeed 3.0) _floatingpawnmovement))
  (:`Released`
    (set `FloatingPawnMovement.MaxSpeed` _defaultmaxspeed _floatingpawnmovement)))

(event `Key|Two`
  (params (Key :type "Key Structure" :default "AnyKey"))
  ;[1 1 1] Follow Capital Ships on 1/2 press
  (:`Pressed`
    (`/Engine/EditorBlueprintResources/StandardMacros.IsValid` (`self.ShipToBlendView`)
      (:`Is Valid`
        (goto _label))
      (:`Is Not Valid`
        (bind _outactors (`GameplayStatics.GetAllActorsOfClass` "/Game/SpaceCombatKit/Blueprints/Ships/SteeringShip_Capital_FireLance.SteeringShip_Capital_FireLance_C"))
        (for _array_element _outactors
          (if (`|EnumEquality` (`/Game/SpaceCombatKit/Blueprints/Ships/BaseClasses/BaseShip.Faction` _array_element) "NewEnumerator1")
            (set `self.ShipToBlendView` _array_element)
            (break)))
        (goto _label_2)))))

(event `Key|NumPadSeven`
  (params (Key :type "Key Structure" :default "AnyKey"))
  ;[1 1 1] Target - If not tracking a ship, Get nearest ship and begin tracking it. If it's valid stop tracking
  (:`Pressed`
    (`/Engine/EditorBlueprintResources/StandardMacros.IsValid` (`self.ShipToTrack`)
      (:`Is Valid`
        (set `self.ShipToTrack` null))
      (:`Is Not Valid`
        (bind _shiptopotentiallytrack1 (`self.GetNearestShip`))
        (set `self.ShipToTrack` _shiptopotentiallytrack1)
        (`self.SetCamerasToFollow`)
        (set `self.CameraToFollowInt` 0)))))

(event `self.ReceiveTick`
  (params (DeltaSeconds :type "Float (single-precision)"))
  (bind _cinecamera (`self.CineCamera`))
  (bind _cameratofollowint (`self.CameraToFollowInt`))
  (bind _cinecamera_2 (`self.CineCamera`))
  (bind _shiptotrack (`self.ShipToTrack`))
  (bind _output (`|GetArrayItem` (`self.CamerasToFollow`) _cameratofollowint))
  ;[1 1 1] Tick
  (`|ExecutionSequence`
    (:`then_0`
      ;[1 1 1] Set focal length based on target focal length, decided by alt fire and zooming in
      (set `CineCameraComponent.CurrentFocalLength` (`KismetMathLibrary.FInterpTo` (`CineCameraComponent.CurrentFocalLength` _cinecamera) (`self.TargetFocal`) (`GameplayStatics.GetWorldDeltaSeconds`) 4.5) _cinecamera))
    (:`then_1`
      ;[1 1 1] If there's a ship to track, track it by setting the rotation of the camera to face that ship + its velocity, and set focus distance to its distance
      (`/Engine/EditorBlueprintResources/StandardMacros.IsValid` _shiptotrack
        (:`Is Valid`
          (`SceneComponent.K2_SetWorldRotation` _cinecamera_2 (`KismetMathLibrary.RInterpTo` (`SceneComponent.K2_GetComponentRotation` _cinecamera_2) (`KismetMathLibrary.FindLookAtRotation` (`SceneComponent.K2_GetComponentLocation` (`self.CineCamera`)) (+ (`self.K2_GetActorLocation` _shiptotrack) (`/Game/SpaceCombatKit/Blueprints/Ships/BaseClasses/BaseShip.GetFlightVelocity` _shiptotrack))) (`GameplayStatics.GetWorldDeltaSeconds`) 5.0) false false)
          (set `CineCameraComponent.FocusSettings` (make `CameraFocusSettings` "Manual" (`self.GetDistanceTo` (`self.ShipToTrack`)) (struct :`RelativeOffset` (0.0 0.0 0.0)) false (struct :`B` 204 :`G` 26 :`R` 102 :`A` 153) true) (`self.CineCamera`)))
        (:`Is Not Valid`
          _))
      (if (`self.BlendLocationToTarget`)
        (`/Engine/EditorBlueprintResources/StandardMacros.IsValid` (`|GetArrayItem` (`self.CamerasToFollow`) _cameratofollowint)
          (:`Is Valid`
            (`self.K2_SetActorLocation` (`KismetMathLibrary.VInterpTo` (`self.K2_GetActorLocation`) (+ (`SceneComponent.K2_GetComponentLocation` _output) (select `bool` (`self.TrackFromFront`) :`true` (+ (* (`SceneComponent.GetForwardVector` _output) 1750.0) (0.0 0.0 250.0)))) (`GameplayStatics.GetWorldDeltaSeconds`) (`self.CameraLocationInterpSpeed`)))))))))

(event `Key|NumPadFive`
  (params (Key :type "Key Structure" :default "AnyKey"))
  ;[1 1 1] Num 5Blend Location To Target
  (:`Pressed`
    (`self.SetCamerasToFollow`)
    (if (`self.BlendLocationToTarget`)
      (set `self.BlendLocationToTarget` false)
      (else
        (set `self.BlendLocationToTarget` true)
        (set `self.CameraToFollowInt` 0)))))

(event `Key|NumPadZero`
  (params (Key :type "Key Structure" :default "AnyKey"))
  (bind _returnvalue (+ (`self.CameraToFollowInt`) 1))
  ;[1 1 1] Change Camera
  (:`Pressed`
    (`self.SetCamerasToFollow`)
    (if (`KismetArrayLibrary.Array_IsValidIndex` (`self.CamerasToFollow`) _returnvalue)
      (set `self.CameraToFollowInt` _returnvalue)
      (else
        (set `self.CameraToFollowInt` 0)))))

(event `Key|Subtract`
  (params (Key :type "Key Structure" :default "AnyKey"))
  ;[1 1 1] Increase / Decrease camera location interp speed
  (:`Pressed`
    (set `self.CameraLocationInterpSpeed` (- (`self.CameraLocationInterpSpeed`) 1.0))))

(event `Key|Add`
  (params (Key :type "Key Structure" :default "AnyKey"))
  ;[1 1 1] Increase / Decrease camera location interp speed
  (:`Pressed`
    (set `self.CameraLocationInterpSpeed` (+ (`self.CameraLocationInterpSpeed`) 1.0))))

(event `Key|NumPadOne`
  (params (Key :type "Key Structure" :default "AnyKey"))
  ;[1 1 1] Toggle track from front/behind
  (:`Pressed`
    (if (`self.TrackFromFront`)
      (set `self.TrackFromFront` false)
      (else
        (set `self.TrackFromFront` true)))))

(fn `GetNearestShip`
  (returns (ShipToPotentiallyTrack1 :type "/Game/SpaceCombatKit/Blueprints/Ships/BaseClasses/BaseShip Object Reference"))
  (locals (DistanceToShips :type "Float (double-precision)" :default 0.0) (ShipToPotentiallyTrack :type "/Game/SpaceCombatKit/Blueprints/Ships/BaseClasses/BaseShip Object Reference"))
  (set `local.DistanceToShips` 500000.0)
  (bind _outactors (`GameplayStatics.GetAllActorsOfClass` "/Game/SpaceCombatKit/Blueprints/Ships/BaseClasses/BaseShip.BaseShip_C"))
  (for _array_element _outactors
    (bind _returnvalue (`self.GetDistanceTo` _array_element))
    (if (< _returnvalue (`local.DistanceToShips`))
      (set `local.DistanceToShips` _returnvalue)
      (set `local.ShipToPotentiallyTrack` _array_element)))
  (return (`local.ShipToPotentiallyTrack`)))

(fn `GetRandomShip`
  (returns (RandomShip :type "/Game/SpaceCombatKit/Blueprints/Ships/BaseClasses/BaseShip Object Reference"))
  (locals (DistanceToShips :type "Float (double-precision)" :default 0.0) (ShipToPotentiallyTrack :type "/Game/SpaceCombatKit/Blueprints/Ships/BaseClasses/BaseShip Object Reference"))
  (bind _outactors (`GameplayStatics.GetAllActorsOfClass` "/Game/SpaceCombatKit/Blueprints/Ships/BaseClasses/BaseShip.BaseShip_C"))
  (return (`|GetArrayItem` _outactors (`KismetMathLibrary.RandomIntegerInRange` 0 (`KismetArrayLibrary.Array_LastIndex` _outactors)))))

(fn `SetBlendView`
  (`PlayerController.SetViewTargetWithBlend` (cast `PlayerController` (`self.GetController`) :!pure true) (cast `/Game/SpaceCombatKit/Blueprints/Ships/BaseClasses/BaseShip` (`self.ShipToBlendView`) :!pure true) 1.0 "VTBlend_Linear" 1.0 true))

(fn `SetCamerasToFollow`
  (`KismetArrayLibrary.Array_Clear` (`self.CamerasToFollow`))
  (for _array_element (`self.K2_GetComponentsByClass` (`self.ShipToTrack`) "/Script/Engine.SceneComponent")
    (cast `CameraComponent` _array_element
      (:`then`
        _)
      (:`CastFailed`
        (cast `CineCameraComponent` _array_element)))
    (`KismetArrayLibrary.Array_AddUnique` (`self.CamerasToFollow`) _array_element)))

(fn `StartTrackingShip`)

(fn `StopBlendView`
  (set `self.ShipToBlendView` null))

(fn `TraceForShip`)

(fn `UserConstructionScript`)