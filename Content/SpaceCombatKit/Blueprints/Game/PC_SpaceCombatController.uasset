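; Player controller for space combat that handles enemy target selection and a Tab-toggled slow-motion mode.
; The Target input sphere-traces from the camera, ignoring the controlled pawn, and sets a hit BaseShip or BaseTurret of another faction as PrimaryTarget.
; A new target replaces any existing aim-prediction marker with a freshly spawned one.
; A trace that hits nothing clears PrimaryTarget but leaves the marker in place.
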(event `self.ReceiveBeginPlay`)

(event `Key|Tab`
  (params (Key :type "Key Structure"))
  ;[1 1 1] Toggle slomo
  (:`Pressed`
    (`/Engine/EditorBlueprintResources/StandardMacros.FlipFlop`
      (:`A`
        (bind _output_get (set `self.SlomoSpeed` 0.1))
        (`KismetSystemLibrary.ExecuteConsoleCommand` (`KismetStringLibrary.Concat_StrStr` "slomo " (`KismetStringLibrary.Conv_DoubleToString` _output_get))))
      (:`B`
        (bind _output_get_2 (set `self.SlomoSpeed` 1.0))
        (`KismetSystemLibrary.ExecuteConsoleCommand` (`KismetStringLibrary.Concat_StrStr` "slomo " (`KismetStringLibrary.Conv_DoubleToString` _output_get_2)))))))

(event `InputAction|Target`
  (params (Key :type "Key Structure"))
  ;[1 1 1] Target pressed - trace for a target
  (:`Pressed`
    (`self.TraceForTarget`)))

(fn `SetAimPredictionTarget`
  (params (ActorToTarget :type "Actor Object Reference"))
  (bind _aimpredictor (`self.AimPredictor`))
  ;[1 1 1] Checks if we already have an aim predictor, and destroy if if we do. Either way spawn a new one and set it's target to our target
  (`/Engine/EditorBlueprintResources/StandardMacros.IsValid` _aimpredictor
    (:`Is Valid`
      (`self.K2_DestroyActor` _aimpredictor))
    (:`Is Not Valid`
      _))
  (bind _returnvalue (`|SpawnActorFromClass` "/Game/SpaceCombatKit/Blueprints/Components/BP_ObjMarker_AimPredict.BP_ObjMarker_AimPredict_C" (`KismetMathLibrary.MakeTransform` (0.0 0.0 0.0)) "Undefined" "OverrideRootScale" (`self.K2_GetPawn`) (cast `Character` ActorToTarget :!pure true) null))
  (set `self.AimPredictor` _returnvalue))

(fn `TraceForTarget`
  (bind _playercameramanager (`self.PlayerCameraManager`))
  (bind _returnvalue (`self.K2_GetActorLocation` _playercameramanager))
  ;[1 1 1] Does a line trace to find targets, based on where the player is looking, ignoring our controlled pawn
  (bind (_outhit _returnvalue_2) (`KismetSystemLibrary.SphereTraceSingle` _returnvalue (+ _returnvalue (* (`self.GetActorForwardVector` _playercameramanager) (`self.TargetDistance`))) 150.0 "TraceTypeQuery1" false (`|MakeArray` (`self.K2_GetPawn`) :!type "Actor Object Reference")))
  ;[1 1 1] If our trace hit something, cast it to BaseShip, check that it's faction isn't equal to our own. If it's not, set it as primary target. If the cast fails, try casting to turret.
  (if _returnvalue_2
    (bind (_bblockinghit _binitialoverlap _time _location _impactpoint _normal _impactnormal _physmat _hitactor) (`GameplayStatics.BreakHitResult` _outhit))
    (bind _asbase_ship (cast `/Game/SpaceCombatKit/Blueprints/Ships/BaseClasses/BaseShip` _hitactor)
      (:`then`
        (if (`|EnumInequality` (`/Game/SpaceCombatKit/Blueprints/Ships/BaseClasses/BaseShip.Faction` _asbase_ship) (`self.Faction`))
          (set `self.PrimaryTarget` _asbase_ship)
          ;[1 1 1] Spawns an aim predictor on the target
          (`self.SetAimPredictionTarget` (`self.PrimaryTarget`) :!label _label)))
      (:`CastFailed`
        (bind _asbase_turret (cast `/Game/SpaceCombatKit/Blueprints/Turrets/BaseTurret` _hitactor))
        (if (`|EnumInequality` (`/Game/SpaceCombatKit/Blueprints/Turrets/BaseTurret.Faction` _asbase_turret) (`self.Faction`))
          (set `self.PrimaryTarget` _asbase_turret)
          (goto _label))))
    (else
      ;[1 1 1] If there's no hit but we have a target, clear it
      (`/Engine/EditorBlueprintResources/StandardMacros.IsValid` (`self.PrimaryTarget`)
        (:`Is Valid`
          (set `self.PrimaryTarget` null))))))

(fn `UserConstructionScript`)