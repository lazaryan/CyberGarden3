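; Team select pawn for the space combat game, letting a starting player join Security or Pirates or spectate.
; Without an HMD, it starts offset behind and above the first PlayerStart, glides in as an intro camera effect and shows the team select widget.
; Keys 1 and 2 request a faction from the game mode, each guarded by DoOnce.
; Key 3 spawns and possesses an observer pawn, preserving control rotation, then destroys itself.
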(event `self.ReceiveTick`
  (params (DeltaSeconds :type "Float (single-precision)"))
  (bind _playerstart (`self.PlayerStart`))
  ;[1 1 1] Tick - Interp our location to the player start for intro animation
  (if (not (`HeadMountedDisplayFunctionLibrary.IsHeadMountedDisplayEnabled`))
    (`self.K2_SetActorLocationAndRotation` (`KismetMathLibrary.VInterpTo` (`self.K2_GetActorLocation`) (`self.K2_GetActorLocation` _playerstart) (`GameplayStatics.GetWorldDeltaSeconds`) 1.0) (`self.K2_GetActorRotation` _playerstart))))

(event `RemoveWidgets` :!signature `self.OnDestroyed`
  (params (DestroyedActor :type "Actor Object Reference"))
  ;[1 1 1] If no HMD, add team select UMG
  ;;[1 1 1] Removes team select widget when we are destroyed
  (`/Engine/EditorBlueprintResources/StandardMacros.IsValid` (stale `self.ReceiveBeginPlay` _returnvalue)
    (:`Is Valid`
      (`Widget.RemoveFromParent` (stale `self.ReceiveBeginPlay` _returnvalue)))))

(event `self.ReceiveBeginPlay`
  ;[1 1 1] Begin play
  ;[1 1 1] Adds an offset and gets the player start to interp into it's location for intro camera effect
  (if (not (`HeadMountedDisplayFunctionLibrary.IsHeadMountedDisplayEnabled`))
    (`self.K2_AddActorWorldOffset` (+ (* (`self.GetActorForwardVector`) -20000.0) (0.0 0.0 6500.0)))
    (bind _outactors (`GameplayStatics.GetAllActorsOfClass` "/Script/Engine.PlayerStart"))
    (set `self.PlayerStart` (`KismetArrayLibrary.Array_Get` _outactors)))
  ;[1 1 1] If no HMD, add team select UMG
  (if (not (`HeadMountedDisplayFunctionLibrary.IsHeadMountedDisplayEnabled`))
    (bind _returnvalue (`|CreateWidget` "/Game/SpaceCombatKit/UMGWidgets/UMG_TeamSelect.UMG_TeamSelect_C" (cast `PlayerController` (`self.GetController`) :!pure true)))
    (`UserWidget.AddToViewport` _returnvalue 0)
    (add `self.OnDestroyed` (delegate `RemoveWidgets`))))

(event `Key|One`
  (params (Key :type "Key Structure" :default "AnyKey"))
  ;[1 1 1] Team select
  (:`Pressed`
    (`/Engine/EditorBlueprintResources/StandardMacros.DoOnce` false
      (:`Completed`
        ;;[1 1 1] Join Security
        (`/Game/SpaceCombatKit/Blueprints/Game/GM_SpaceCombatGameMode.AssignFactionToPC` (cast `/Game/SpaceCombatKit/Blueprints/Game/GM_SpaceCombatGameMode` (`GameplayStatics.GetGameMode`) :!pure true) "NewEnumerator2" (cast `PlayerController` (`self.GetController`) :!pure true))))))

(event `Key|Two`
  (params (Key :type "Key Structure" :default "AnyKey"))
  ;[1 1 1] Team select
  (:`Pressed`
    (`/Engine/EditorBlueprintResources/StandardMacros.DoOnce` false
      (:`Completed`
        ;;[1 1 1] Join Pirates
        (`/Game/SpaceCombatKit/Blueprints/Game/GM_SpaceCombatGameMode.AssignFactionToPC` (cast `/Game/SpaceCombatKit/Blueprints/Game/GM_SpaceCombatGameMode` (`GameplayStatics.GetGameMode`) :!pure true) "NewEnumerator1" (cast `PlayerController` (`self.GetController`) :!pure true))))))

(event `Key|Three`
  (params (Key :type "Key Structure" :default "AnyKey"))
  ;[1 1 1] Spawns a PawnObserver - stores control rotation and controller to apply rotation to controller after possession
  (:`Pressed`
    (`self.RemoveWidgets` null)
    (bind _returnvalue (`|SpawnActorFromClass` "/Game/SpaceCombatKit/Blueprints/Game/Pawn_Observer.Pawn_Observer_C" (`self.GetTransform`) "AlwaysSpawn" "OverrideRootScale"))
    (bind _output_get (set `self.TempControlRotation` (`self.GetControlRotation`)))
    (bind _output_get_2 (set `self.TempController` (`self.GetController`)))
    (`Controller.Possess` _output_get_2 _returnvalue)
    (`Controller.SetControlRotation` _output_get_2 _output_get)
    (`self.K2_DestroyActor`)))

(fn `UserConstructionScript`)