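; BP_ObjectiveMarker is a Space Combat Kit objective marker drawn with a material billboard in a configurable color.
; The construction script passes its red, blue and green variables to the UpdateColor event.
; UpdateColor creates a dynamic material instance from the billboard's first material and writes the three values as separate scalar parameters.
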(event `UpdateColor`
  (params (RedValue :type "Float (double-precision)") (BlueValue :type "Float (double-precision)") (GreenValue :type "Float (double-precision)"))
  (bind _materialbillboard1 (`self.MaterialBillboard1`))
  ;[1 1 1] Updates the colour based on Red, Blue, and Green values
  (bind _returnvalue (`PrimitiveComponent.CreateDynamicMaterialInstance` _materialbillboard1 0 (`PrimitiveComponent.GetMaterial` _materialbillboard1 0)))
  (`MaterialInstanceDynamic.SetScalarParameterValue` _returnvalue "red" RedValue)
  (`MaterialInstanceDynamic.SetScalarParameterValue` _returnvalue "blue" BlueValue)
  (`MaterialInstanceDynamic.SetScalarParameterValue` _returnvalue "green" GreenValue))

(fn `UserConstructionScript`
  (`self.UpdateColor` (`self.RedValue`) (`self.BlueValue`) (`self.GreenValue`)))