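; Steering behaviour component for AI-flown BaseShips in space combat, providing seek, flee, pursue, evade, arrive, wander, follow, separation and spline path behaviours.
; Behaviours return forces that AddAISteeringForce weights and sums; Tick adds sphere-based trace avoidance, skipping player-controlled or locked ships.
; The force is cone-limited to a maximum turn angle, truncated and mass-scaled, then drives CharacterMovement velocity and interpolated rotation with optional banking.
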(event `self.ReceiveBeginPlay`
  ;[1 1 1] Make sure ship is facing forward at start of play
  (set `self.Velocity` (`Actor.GetActorForwardVector` (`self.GetOwner`))))

(event `self.ReceiveTick`
  (params (DeltaSeconds :type "Float (single-precision)"))
  (bind _asbase_ship (cast `/Game/SpaceCombatKit/Blueprints/Ships/BaseClasses/BaseShip` (`self.GetOwner`) :!pure true))
  (cast `PlayerController` (`Pawn.GetController` _asbase_ship)
    (:`CastFailed`
      (if (not (`/Game/SpaceCombatKit/Blueprints/Ships/BaseClasses/BaseShip.ControlsLocked` _asbase_ship))
        (`self.Move` DeltaSeconds)))))

(fn `AddAISteeringForce`
  (params (SteeringForce :type "Vector Structure") (Weight :type "Float (double-precision)"))
  (set `self.AISteeringForce` (+ (`self.AISteeringForce`) (* SteeringForce Weight))))

(fn `AdjustRawSteeringForce`
  (params (Force :type "Vector Structure"))
  (returns (ReturnValue :type "Vector Structure"))
  (locals (MaxAdjustedSpeed :type "Float (double-precision)") (Range :type "Float (double-precision)") (Cosine :type "Float (double-precision)"))
  (if (== Force (0.0 0.0 0.0) :`ErrorTolerance` 0.1)
    (return Force)
    (else
      (bind _returnvector (`self.LimitDeviationAngle` true Force (`KismetMathLibrary.DegCos` (`self.Maximum Turn angle`)) (`Actor.GetActorForwardVector` (`self.GetOwner`))))
      (return _returnvector))))

(fn `ApplySteeringForce`
  (params (Force :type "Vector Structure") (DeltaTime :type "Float (double-precision)"))
  (locals (AdjustedForce :type "Vector Structure") (ClippedForce :type "Vector Structure") (NewAcceleration :type "Vector Structure") (NewVelocity :type "Vector Structure"))
  (bind _returnvalue (`self.GetOwner`))
  (bind _returnvalue_2 (`self.GetOwner`))
  (bind _steering (`self.Steering`))
  (bind _returnvalue_3 (`self.AdjustRawSteeringForce` Force))
  ;[1 1 1] Can set any behaviour here. Should change depending on circumstance. Steering = all behaviours added up and then truncated. Can put weights onto individual behaviours for better results
  (bind _output_get (set `self.Steering` (/ (`self.TruncateVector` _returnvalue_3 (`self.MaxSpeed`)) (`self.Mass`))))
  ;[1 1 1] Truncate velocity so it's within max speed.
  (bind _output_get_2 (set `self.Velocity` (`self.TruncateVector` (+ (`self.Velocity`) _output_get) (`KismetMathLibrary.VSize` (`self.DesiredVelocity`)))))
  ;[1 1 1] Set actor location to new position
  (bind _asbase_ship (cast `/Game/SpaceCombatKit/Blueprints/Ships/BaseClasses/BaseShip` (`self.GetOwner`)))
  (set `MovementComponent.Velocity` _output_get_2 (`Character.CharacterMovement` _asbase_ship)) ; Use character movement to move ship.\n\nAlternatively you can set actor location to \n(Velocity * DeltaTime) + Actor Location.
  ;[1 1 1] Rotate to new facing
  (bind _asbase_ship_2 (cast `/Game/SpaceCombatKit/Blueprints/Ships/BaseClasses/BaseShip` (`self.GetOwner`)))
  (if (not (`/Game/SpaceCombatKit/Blueprints/Ships/BaseClasses/BaseShip.ControlsLocked` _asbase_ship_2))
    (if (`self.BankingRoll`)
      (bind _output_get_3 (set `self.CurrentRoll` (`KismetMathLibrary.FInterpTo` (`self.CurrentRoll`) (.roll (`KismetMathLibrary.MakeRotationFromAxes` (`Actor.GetActorForwardVector` _returnvalue_2) (`Actor.GetActorRightVector` _returnvalue_2) (`KismetMathLibrary.Normal` (`self.Steering`)))) DeltaTime (`self.TurnRate`)))))
    (`Actor.K2_SetActorRotation` _returnvalue (`KismetMathLibrary.MakeRotator` _output_get_3 (.pitch (`KismetMathLibrary.RInterpTo` (`Actor.K2_GetActorRotation` _returnvalue) (`KismetMathLibrary.MakeRotFromX` (select `bool` (`self.Plane-Like Rotation`) :`false` _steering :`true` (+ _steering (`self.Velocity`)))) DeltaTime (`self.TurnRate`))) (.yaw (`KismetMathLibrary.RInterpTo` (`Actor.K2_GetActorRotation` _returnvalue) (`KismetMathLibrary.MakeRotFromX` (select `bool` (`self.Plane-Like Rotation`) :`false` _steering :`true` (+ _steering (`self.Velocity`)))) DeltaTime (`self.TurnRate`)))) false)))

(fn `Arrive`
  (params (Target :type "Vector Structure") (SlowDownDistance :type "Float (double-precision)" :default 1500.0))
  (returns (Steering :type "Vector Structure"))
  (locals (Distance :type "Float (double-precision)") (SlowDistance :type "Float (double-precision)"))
  ;[1 1 1] Distance from target
  (set `local.SlowDistance` SlowDownDistance)
  (bind _output_get (set `local.Distance` (`KismetMathLibrary.VSize` (- Target (`Actor.K2_GetActorLocation` (`self.GetOwner`))))))
  (if (< _output_get (`local.SlowDistance`))
    ;[1 1 1] Slow down
    (set `self.DesiredVelocity` (* (* (`KismetMathLibrary.Normal` (`self.DesiredVelocity`)) (`self.MaxSpeed`)) (/ (`local.Distance`) (`local.SlowDistance`))))
    (else
      ;[1 1 1] Go full speed
      (set `self.DesiredVelocity` (* (`KismetMathLibrary.Normal` (`self.DesiredVelocity`)) (`self.MaxSpeed`)))))
  (return (- (`self.DesiredVelocity`) (`self.Velocity`))))

(fn `CheckForObstructions`
  (returns (Avoidance :type "Vector Structure") (Obstruction :type Boolean))
  (locals (AvoidanceForce :type "Vector Structure") (DynamicLength :type "Float (double-precision)"))
  (bind _returnvalue (`self.GetOwner`))
  (bind _returnvalue_2 (`Actor.K2_GetActorLocation` _returnvalue))
  (bind _returnvalue_3 (* (`self.Velocity`) (`local.DynamicLength`)))
  ;[1 1 1] Basic avoidance to work with spheres, using an interface to find out which objects to avoid, which gives the actor an avoidance sphere
  (set `local.DynamicLength` (/ (`KismetMathLibrary.VSize` (`self.Velocity`)) (`self.MaxSpeed`)))
  (bind _outhit (`KismetSystemLibrary.LineTraceSingle` _returnvalue_2 (+ _returnvalue_2 _returnvalue_3) (enumliteral `ETraceTypeQuery` "TraceTypeQuery3") false (`|MakeArray` _returnvalue)))
  (bind (_bblockinghit _binitialoverlap _time _location _impactpoint _normal _impactnormal _physmat _hitactor) (`GameplayStatics.BreakHitResult` _outhit))
  (if _bblockinghit
    (bind _sphere (message `/Game/SpaceCombatKit/Blueprints/Components/SteeringAvoidanceInterface.GetAvoidanceSphere` _hitactor))
    (bind _output_get (set `local.AvoidanceForce` (* (`KismetMathLibrary.Normal` (- _returnvalue_3 (`KismetSystemLibrary.GetComponentBounds` _sphere))) (`self.MaxAvoidanceForce`))))
    (return _output_get true)
    (else
      (return (0.0 0.0 0.0) false))))

(fn `Evade`
  (params (TargetShip :type "/Game/SpaceCombatKit/Blueprints/Ships/BaseClasses/BaseShip Object Reference"))
  (returns (Steering :type "Vector Structure"))
  (bind _steering (`self.Flee` (`self.GetTargetFuturePosition` TargetShip)))
  (return _steering))

(fn `Flee`
  (params (Target :type "Vector Structure"))
  (returns (Steering :type "Vector Structure"))
  (locals (SteeringForce :type "Vector Structure"))
  (bind _output_get (set `self.DesiredVelocity` (* (`KismetMathLibrary.Normal` (- (`Actor.K2_GetActorLocation` (`self.GetOwner`)) Target)) (`self.MaxSpeed`))))
  (bind _output_get_2 (set `local.SteeringForce` (- _output_get (`self.Velocity`))))
  (return _output_get_2))

(fn `FollowPath`
  (params (SplinePath :type "/Game/SpaceCombatKit/Blueprints/Components/BP_SplinePath Object Reference") (DistanceForPointChange :type "Float (double-precision)" :default 500.0) (`ResetWhenFinished?` :type Boolean :default true))
  (returns (Steering :type "Vector Structure"))
  (locals (TargetPoint :type "Vector Structure") (OutSteering :type "Vector Structure"))
  (bind _spline (`/Game/SpaceCombatKit/Blueprints/Components/BP_SplinePath.Spline` SplinePath))
  (`/Engine/EditorBlueprintResources/StandardMacros.IsValid` SplinePath
    (:`Is Valid`
      ;[1 1 1] Set target destination as current spline point location
      (bind _output_get (set `local.TargetPoint` (`SplineComponent.GetLocationAtSplinePoint` _spline (`self.CurrentSplineIndex`) "World")))
      ;[1 1 1] If the distance between the ship and the current path point is less than the DistanceForPointChange, go to the next point
      (bind _steering (`self.Seek` _output_get))
      (set `local.OutSteering` _steering)
      (if (< (`KismetMathLibrary.VSize` (- (`local.TargetPoint`) (`Actor.K2_GetActorLocation` (`self.GetOwner`)))) DistanceForPointChange)
        (`/Engine/EditorBlueprintResources/StandardMacros.IncrementInt` (`self.CurrentSplineIndex`)
          (:`  `
            ;[1 1 1] If the node index is higher than the number of nodes, and we want to reset, reset to 0 index
            (if (and (>= (`self.CurrentSplineIndex`) (`SplineComponent.GetNumberOfSplinePoints` _spline)) `ResetWhenFinished?`)
              (set `self.CurrentSplineIndex` 0)))))
      ;[1 1 1] Return the steering to the point
      (return (`local.OutSteering`)))))

(fn `FollowShip`
  (params (TargetShip :type "/Game/SpaceCombatKit/Blueprints/Ships/BaseClasses/BaseShip Object Reference") (FollowDistance :type "Float (double-precision)"))
  (returns (Steering :type "Vector Structure"))
  (bind _steering (`self.Seek` (+ (`Actor.K2_GetActorLocation` TargetShip) (* (* (`KismetMathLibrary.Normal` (`/Game/SpaceCombatKit/Blueprints/Ships/BaseClasses/BaseShip.GetShipVelocity` TargetShip)) -1.0) FollowDistance))))
  (bind _outsteering (`self.Separation` (`self.SeparationRadius`)))
  (return (+ _outsteering _steering)))

(fn `GetParallelComponent`
  (params (Vector :type "Vector Structure") (UnitBasis :type "Vector Structure"))
  (returns (Result :type "Vector Structure"))
  (locals (Projection :type "Float (double-precision)"))
  (bind _output_get (set `local.Projection` (`KismetMathLibrary.Dot_VectorVector` Vector UnitBasis)))
  (return (* UnitBasis _output_get)))

(fn `GetPerpendicularComponent`
  (params (Vector :type "Vector Structure") (UnitBasis :type "Vector Structure"))
  (returns (Result :type "Vector Structure"))
  (return (- Vector (`self.GetParallelComponent` Vector UnitBasis))))

(fn `GetTargetFuturePosition`
  (params (TargetShip :type "/Game/SpaceCombatKit/Blueprints/Ships/BaseClasses/BaseShip Object Reference"))
  (returns (FuturePosition :type "Vector Structure"))
  (locals (TargetMaxSpeed :type "Float (double-precision)"))
  (bind _component (`/Game/SpaceCombatKit/Blueprints/Ships/BaseClasses/BaseShip.GetSteeringComponent` TargetShip))
  (bind _returnvalue (`Actor.K2_GetActorLocation` TargetShip))
  ;[1 1 1] Find targets max speed for all types of movements
  (`/Engine/EditorBlueprintResources/StandardMacros.IsValid` _component
    (:`Is Valid`
      (set `local.TargetMaxSpeed` (`/Game/SpaceCombatKit/Blueprints/Components/BPC_SteeringBehaviourComponent.MaxSpeed` _component)))
    (:`Is Not Valid`
      (set `local.TargetMaxSpeed` (`CharacterMovementComponent.MaxFlySpeed` (`Character.CharacterMovement` TargetShip)))))
  (return (+ (* (`/Game/SpaceCombatKit/Blueprints/Ships/BaseClasses/BaseShip.GetShipVelocity` TargetShip) (/ (`KismetMathLibrary.VSize` (- _returnvalue (`Actor.K2_GetActorLocation` (`self.GetOwner`)))) (`local.TargetMaxSpeed`))) _returnvalue)))

(fn `LimitDeviationAngle`
  (params (Inside :type Boolean) (Source :type "Vector Structure") (CosineOfConeAngle :type "Float (double-precision)") (Basis :type "Vector Structure"))
  (returns (ReturnVector :type "Vector Structure"))
  (locals (SourceLength :type "Float (double-precision)") (Direction :type "Vector Structure") (CosineOfSourceAngle :type "Float (double-precision)") (Perpendicular :type "Vector Structure") (UnitPerpendicular :type "Vector Structure") (PerpDist :type "Float (double-precision)") (c0 :type "Vector Structure") (c1 :type "Vector Structure"))
  ;[1 1 1] Immediately return zero length input vectors
  (bind _output_get (set `local.SourceLength` (`KismetMathLibrary.VSize` Source)))
  (if (== _output_get 0.0)
    (return Source)
    (else
      ;[1 1 1] Measure angular deviation of source from basis
      (bind _output_get_2 (set `local.Direction` (/ Source (`local.SourceLength`))))
      (set `local.CosineOfSourceAngle` (`KismetMathLibrary.Dot_VectorVector` _output_get_2 Basis))
      ;[1 1 1] Return source if it is already within the angle
      (if Inside
        (if (>= (`local.CosineOfSourceAngle`) CosineOfConeAngle)
          ;[1 1 1] Source is inside cone, return
          (return Source)
          (else
            _))
        (elif (<= (`local.CosineOfSourceAngle`) CosineOfConeAngle)
          ;[1 1 1] Source is outside cone, return
          (return Source)
          (else
            _)))
      ;[1 1 1] Find the portion of source that is perpendicular to basis
      (bind _output_get_3 (set `local.Perpendicular` (`self.GetPerpendicularComponent` Source Basis)))
      ;[1 1 1] construct a new vector whose length equals the source vector, and lies on the intersection of a plane (formed the source and basis vectors) and a cone (whose axis is "basis" and whose angle corresponds to cosineOfConeAngle)
      (bind _output_get_4 (set `local.PerpDist` (`KismetMathLibrary.Sqrt` (- 1.0 (* CosineOfConeAngle CosineOfConeAngle)))))
      (bind _output_get_5 (set `local.c0` (* Basis CosineOfConeAngle)))
      (bind _output_get_6 (set `local.c1` (* (`KismetMathLibrary.Normal` _output_get_3) _output_get_4)))
      (return (* (+ _output_get_5 _output_get_6) (`local.SourceLength`))))))

(fn `Move`
  (params (DeltaTime :type "Float (double-precision)"))
  (bind (_avoidance _obstruction) (`self.CheckForObstructions`))
  (if _obstruction
    (`self.ApplySteeringForce` _avoidance DeltaTime)
    (else
      (`self.ApplySteeringForce` (+ _avoidance (`self.AISteeringForce`)) DeltaTime))))

(fn `Pursue`
  (params (TargetShip :type "/Game/SpaceCombatKit/Blueprints/Ships/BaseClasses/BaseShip Object Reference"))
  (returns (Steering :type "Vector Structure"))
  ;[1 1 1] Seek after the predicted position
  (bind _steering (`self.Seek` (`self.GetTargetFuturePosition` TargetShip)))
  (return _steering))

(fn `ScalarRandomWalk`
  (params (Initial :type "Float (double-precision)") (WalkSpeed :type "Float (double-precision)") (Min :type "Float (double-precision)") (Max :type "Float (double-precision)"))
  (returns (ReturnValue :type "Float (double-precision)"))
  (locals (Next :type "Float (double-precision)"))
  ;[1 1 1] Random walk algorithm for wander behaviour
  (return (`KismetMathLibrary.FClamp` (+ Initial (* (- (* (`KismetMathLibrary.RandomFloat`) 2.0) 1.0) WalkSpeed)) Min Max)))

(fn `Seek`
  (params (Target :type "Vector Structure"))
  (returns (Steering :type "Vector Structure"))
  (locals (SteeringForce :type "Vector Structure"))
  (set `self.DesiredVelocity` (* (`KismetMathLibrary.Normal` (- Target (`Actor.K2_GetActorLocation` (`self.GetOwner`)))) (`self.MaxSpeed`)))
  (bind _output_get (set `local.SteeringForce` (- (`self.DesiredVelocity`) (`self.Velocity`))))
  (return _output_get))

(fn `Separation`
  (params (SeparationRadius :type "Float (double-precision)" :default 1000.0))
  (returns (OutSteering :type "Vector Structure"))
  (locals (NumShips :type Integer) (OutForce :type "Vector Structure") (TotalForce :type "Vector Structure"))
  (bind _returnvalue (`self.GetOwner`))
  (bind _outactors (`GameplayStatics.GetAllActorsOfClass` "/Game/SpaceCombatKit/Blueprints/Ships/BaseClasses/BaseShip.BaseShip_C"))
  (for _array_element _outactors
    (if (!= _array_element _returnvalue)
      (bind _returnvalue_2 (`Actor.K2_GetActorLocation` _array_element))
      (bind _returnvalue_3 (`KismetMathLibrary.VSize` (- _returnvalue_2 (`Actor.K2_GetActorLocation` _returnvalue))))
      (if (and (< _returnvalue_3 SeparationRadius) (> _returnvalue_3 0.0))
        (`/Engine/EditorBlueprintResources/StandardMacros.IncrementInt` (`local.NumShips`)
          (:`  `
            (set `local.TotalForce` (+ (`local.TotalForce`) (/ (- (`Actor.K2_GetActorLocation` (`self.GetOwner`)) _returnvalue_2) SeparationRadius))))))))
  ;[1 1 1] If there are any ships to separate from, do it, else return a zerovector
  (if (> (`local.NumShips`) 0)
    (bind _output_get (set `local.TotalForce` (/ (`local.TotalForce`) (`local.NumShips`))))
    (return (* _output_get (`self.MaxSeparation`)))
    (else
      (return (0.0 0.0 0.0)))))

(fn `TruncateVector`
  (params (Vector :type "Vector Structure") (MaxValue :type "Float (double-precision)"))
  (returns (OutVector :type "Vector Structure"))
  (locals (Scale :type "Float (double-precision)") (ScaledVector :type "Vector Structure"))
  ;[1 1 1] Truncate vector so it's within the max speed
  (if (!= Vector (0.0 0.0 0.0))
    (bind _output_get (set `local.Scale` (/ MaxValue (`KismetMathLibrary.VSize` Vector))))
    (bind _output_get_2 (set `local.Scale` (`KismetMathLibrary.SelectFloat` _output_get 1.0 (< _output_get 1.0))))
    (bind _output_get_3 (set `local.ScaledVector` (* Vector _output_get_2)))
    (return _output_get_3)
    (else
      (return Vector))))

(fn `Wander`
  (params (MaxLatitudeSide :type "Float (double-precision)" :default 2.0) (MaxLatitudeUp :type "Float (double-precision)" :default 2.0))
  (returns (Steering :type "Vector Structure"))
  (locals (CircleCentre :type "Vector Structure") (Displacement :type "Vector Structure") (WanderVector :type "Vector Structure") (RandomSide :type "Float (double-precision)") (RandomUp :type "Float (double-precision)"))
  ;[1 1 1] Get random walks for up and side
  (bind _returnvalue (`self.ScalarRandomWalk` (`self.WanderAngle`) (`KismetMathLibrary.VSize` (`self.DesiredVelocity`)) (* MaxLatitudeSide -1.0) MaxLatitudeSide))
  (set `local.RandomSide` _returnvalue)
  (bind _returnvalue_2 (`self.ScalarRandomWalk` (`self.WanderAngleZ`) (`KismetMathLibrary.VSize` (`self.DesiredVelocity`)) (* MaxLatitudeUp -1.0) MaxLatitudeUp))
  (bind _output_get (set `local.RandomUp` _returnvalue_2))
  (bind _output_get_2 (set `local.WanderVector` (- (`KismetMathLibrary.MakeVector` (.x (`self.DesiredVelocity`)) (* (.y (`self.DesiredVelocity`)) (`local.RandomSide`)) (* (.z (`self.DesiredVelocity`)) _output_get)) (`self.Velocity`))))
  (return _output_get_2))