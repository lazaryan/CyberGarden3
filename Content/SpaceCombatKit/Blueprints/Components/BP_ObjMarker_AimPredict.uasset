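; Objective marker actor that shows a lead-aim point for its owning ship's AimTarget in space combat.
; Each tick it moves itself to the predicted target position, destroying itself if either the ship or target is invalid.
; Prediction is linear: target velocity times travel time from the first primary weapon's projectile speed, ignoring shooter velocity.
; BaseShip targets supply ship velocity; other actors use standard actor velocity.
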(event `self.ReceiveBeginPlay`
  ;[1 1 1] Begin play, set the ship that owns us so we can get it's weapons range
  (bind _asbase_ship (cast `/Game/SpaceCombatKit/Blueprints/Ships/BaseClasses/BaseShip` (`self.GetOwner`)))
  (set `self.OwningShip` _asbase_ship))

(event `self.ReceiveTick`
  (params (DeltaSeconds :type "Float (single-precision)"))
  (`/Engine/EditorBlueprintResources/StandardMacros.IsValid` (`self.OwningShip`)
    (:`Is Valid`
      (`/Engine/EditorBlueprintResources/StandardMacros.IsValid` (`self.AimTarget`)
        (:`Is Valid`
          ;[1 1 1] Sets our location to the prediction position of the target
          (`self.K2_SetActorRelativeLocation` (`self.GetPredictedPosition`)))
        (:`Is Not Valid`
          ;[1 1 1] Our target is no longer valid. Destroy ourselves
          (`self.K2_DestroyActor` :!label _label))))
    (:`Is Not Valid`
      (goto _label))))

(fn `GetBulletTravelTimeToTarget`
  (returns (TravelTIme :type "Float (double-precision)"))
  (bind _item (`KismetArrayLibrary.Array_Get` (`/Game/SpaceCombatKit/Blueprints/Ships/BaseClasses/BaseShip.PrimaryWeapons` (`self.OwningShip`))))
  (return (/ (`KismetMathLibrary.VSize` (- (`self.K2_GetActorLocation` (`self.AimTarget`)) (`self.K2_GetActorLocation` _item))) (`/Game/SpaceCombatKit/Blueprints/Weapons/BaseWeapon.ProjectileSpeed` _item))))

(fn `GetPredictedPosition`
  (returns (PredictedPosition :type "Vector Structure"))
  (bind _aimtarget (`self.AimTarget`))
  (bind _asbase_ship (cast `/Game/SpaceCombatKit/Blueprints/Ships/BaseClasses/BaseShip` _aimtarget)
    (:`then`
      (return (+ (`self.K2_GetActorLocation` _asbase_ship) (* (`/Game/SpaceCombatKit/Blueprints/Ships/BaseClasses/BaseShip.GetShipVelocity` _asbase_ship) (`self.GetBulletTravelTimeToTarget`)))))
    (:`CastFailed`
      (return (+ (`self.K2_GetActorLocation` _aimtarget) (* (`self.GetVelocity` _aimtarget) (`self.GetBulletTravelTimeToTarget`)))))))

(fn `UserConstructionScript`
  (`parent.UserConstructionScript`))