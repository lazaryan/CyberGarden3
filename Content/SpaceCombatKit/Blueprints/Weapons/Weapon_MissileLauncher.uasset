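; Missile launcher weapon that fires homing missiles from muzzle sockets on its mesh.
; Each shot cycles to the next socket, playing the fire sound and spawning the projectile there with the parent pawn as instigator.
; A forward sphere trace from the "Muzzle" socket then sets any turret or non-capital pawn hit as the missile's homing target.
; BeginPlay and Reload also reset the muzzle slot count.
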(event `self.Reload`
  ;[1 1 1] Sets the muzzle slots so we can get the muzzle vector to launch with an offset
  ;;[1 1 1] After reloading, set muzzle slots to max ammo in mag -1
  (`parent.Reload`)
  (set `self.MuzzleSlots` (- (`self.MaxAmmoInMag`) 1)))

(event `self.ReceiveBeginPlay`
  ;[1 1 1] Sets the muzzle slots so we can get the muzzle vector to launch with an offset
  ;;[1 1 1] Begin play - set muzzle slots to max ammo in mag -1
  (`parent.ReceiveBeginPlay`)
  (set `self.MuzzleSlots` (`KismetArrayLibrary.Array_Length` (`SceneComponent.GetAllSocketNames` (`self.WeaponMesh`)))))

(event `self.SpawnProjectile`
  (bind (_returnvalue_location _returnvalue_rotation) (`KismetMathLibrary.BreakTransform` (`SceneComponent.GetSocketTransform` (`self.WeaponMesh`) "Muzzle" "RTS_World")))
  (bind _aspawn (cast `Pawn` (`self.GetParentActor`) :!pure true))
  ;[1 1 1] Spawns a projectile and then traces to see if the missile launcher was aiming at a pawn or turret - if it was, set that as the missiles homing target
  (bind _socketname (`self.GetAndSetMuzzleIndex`))
  (bind (_returnvalue_location_2 _returnvalue_rotation_2) (`KismetMathLibrary.BreakTransform` (`SceneComponent.GetSocketTransform` (`self.WeaponMesh`) _socketname "RTS_World")))
  (`GameplayStatics.SpawnSoundAtLocation` (`self.FireSound`) _returnvalue_location_2 (struct) 0.15 0.5 0.0 "/Game/SpaceCombatKit/Sounds/Weapons/WeaponsFireAttenuation.WeaponsFireAttenuation")
  (bind _returnvalue (`|SpawnActorFromClass` (`self.Projectile`) (`KismetMathLibrary.MakeTransform` _returnvalue_location_2 _returnvalue_rotation_2) "Undefined" "OverrideRootScale" null 40.0 10.0 500.0 _aspawn))
  (bind _outhit (`KismetSystemLibrary.SphereTraceSingle` _returnvalue_location (+ _returnvalue_location (* (`KismetMathLibrary.GetForwardVector` _returnvalue_rotation) 5000.0)) 20.0 "TraceTypeQuery1" false (`|MakeArray` _aspawn :!type "Actor Object Reference")))
  (bind _asbase_turret (cast `/Game/SpaceCombatKit/Blueprints/Turrets/BaseTurret` (`.HitActor` (`GameplayStatics.BreakHitResult` _outhit)))
    (:`then`
      (bind _projectilemovement (`/Game/SpaceCombatKit/Blueprints/Projectiles/Proj_Missile.ProjectileMovement` (cast `/Game/SpaceCombatKit/Blueprints/Projectiles/Proj_Missile` _returnvalue :!pure true)))
      (set `ProjectileMovementComponent.HomingTargetComponent` (`self.K2_GetRootComponent` _asbase_turret) _projectilemovement))
    (:`CastFailed`
      (bind _aspawn_2 (cast `Pawn` (`.HitActor` (`GameplayStatics.BreakHitResult` _outhit))))
      (cast `/Game/SpaceCombatKit/Blueprints/Ships/BaseClasses/BaseCapital` (`.HitActor` (`GameplayStatics.BreakHitResult` _outhit)) ; Don't bother homing capitals
        (:`CastFailed`
          (set `ProjectileMovementComponent.HomingTargetComponent` (`self.K2_GetRootComponent` _aspawn_2) _projectilemovement))))))

(fn `GetAndSetMuzzleIndex`
  (returns (SocketName :type Name))
  (locals (TempSocketName :type Name))
  (bind _returnvalue (`SceneComponent.GetAllSocketNames` (`self.WeaponMesh`)))
  (bind _returnvalue_2 (+ (`self.CurrentMuzzleIndex`) 1))
  (set `local.TempSocketName` (`|GetArrayItem` _returnvalue (`self.CurrentMuzzleIndex`)))
  (if (`KismetArrayLibrary.Array_IsValidIndex` _returnvalue _returnvalue_2)
    (set `self.CurrentMuzzleIndex` _returnvalue_2)
    (return (`local.TempSocketName`))
    (else
      (set `self.CurrentMuzzleIndex` 0)
      (return (`local.TempSocketName`)))))

(fn `UserConstructionScript`
  (`parent.UserConstructionScript`))