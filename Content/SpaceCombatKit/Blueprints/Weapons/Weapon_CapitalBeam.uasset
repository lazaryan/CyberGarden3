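; Capital ship beam weapon that fires a timed, colored particle beam and repeatedly damages the ship it hits.
; SpawnProjectile activates the emitter and opens a gate for about two seconds, during which Tick line-traces forward to update beam endpoint, length and width.
; On hitting a BaseShip, a distance-based delay mimics beam travel time.
; A second gate then spawns attached explosions and applies damage at short intervals until a timer closes it.
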(event `self.ReceiveBeginPlay`
  ;[1 1 1] On begin play, set the beam color
  (`parent.ReceiveBeginPlay`)
  (`ParticleSystemComponent.SetVectorParameter` (`self.ParticleSystem`) "color" (`self.BeamRGBColor`)))

(event `self.ReceiveTick`
  (params (DeltaSeconds :type "Float (single-precision)"))
  (bind _returnvalue (`self.K2_GetActorLocation`))
  (bind _particlesystem (`self.ParticleSystem`))
  (bind _returnvalue_2 (+ _returnvalue (* (`self.GetActorForwardVector`) (`self.BeamLength`))))
  ;[1 1 1] Updates the beam emitter location if it's active
  (`parent.ReceiveTick` DeltaSeconds)
  (`|ExecutionSequence`
    (:`then_0`
      (`/Engine/EditorBlueprintResources/StandardMacros.Gate` true :!label _label
        (:`Exit`
          ;[1 1 1] Trace forward. If he hit something, set that as the end of the beam emitter. If not, forward vector * distance
          (bind (_outhit _returnvalue_3) (`KismetSystemLibrary.LineTraceSingle` _returnvalue _returnvalue_2 "TraceTypeQuery1"))
          (bind _returnvalue_4 (select `bool` _returnvalue_3 :`false` _returnvalue_2 :`true` (`.Location` (`GameplayStatics.BreakHitResult` _outhit))))
          (`ParticleSystemComponent.SetBeamTargetPoint` _particlesystem 0 _returnvalue_4 0)
          (bind _returnvalue_5 (`KismetMathLibrary.VSize` (- _returnvalue _returnvalue_4)))
          (`ParticleSystemComponent.SetFloatParameter` _particlesystem "distance" _returnvalue_5)
          (`ParticleSystemComponent.SetFloatParameter` _particlesystem "taperscale" (`self.BeamWidth`))
          (bind _asbase_ship (cast `/Game/SpaceCombatKit/Blueprints/Ships/BaseClasses/BaseShip` (`.HitActor` (`GameplayStatics.BreakHitResult` _outhit))))
          (bind _output_get (set `self.HitShip` _asbase_ship))
          (`|ExecutionSequence`
            (:`then_0`
              (`/Engine/EditorBlueprintResources/StandardMacros.DoOnce` false :!label _label_2
                (:`Completed`
                  ;;[1 1 1] Spawns an explosion and does damage every X seconds while the emitter is still active
                  (`KismetSystemLibrary.Delay` (/ _returnvalue_5 30000.0)) ; Delays until the beam hits the target
                  (set `self.DelayUntilSparks` 0.0)
                  (goto _label_3 :!via `Open`))))
            (:`then_1`
              (`KismetSystemLibrary.Delay` 1.5) ; Delays until the beam ends
              (goto _label_3 :!via `Close`))))))
    (:`then_1`
      (`/Engine/EditorBlueprintResources/StandardMacros.Gate` true :!label _label_3
        (:`Exit`
          (`KismetSystemLibrary.Delay` (`self.DelayUntilSparks`))
          (bind _returnvalue_6 (`GameplayStatics.SpawnEmitterAttached` "/Game/SpaceCombatKit/Particles/StarterContent/Particles/P_Explosion.P_Explosion" (`/Game/SpaceCombatKit/Blueprints/Ships/BaseClasses/BaseShip.ShipMesh` _output_get) "None" (`.Location` (`GameplayStatics.BreakHitResult` _outhit)) (`KismetMathLibrary.Conv_VectorToRotator` (`.Normal` (`GameplayStatics.BreakHitResult` _outhit))) "KeepWorldPosition"))
          (`GameplayStatics.ApplyDamage` _output_get (`self.ProjectileDamage`))
          (`SceneComponent.SetWorldScale3D` _returnvalue_6 (2.0 2.0 2.0))
          (set `self.DelayUntilSparks` 0.1))))))

(event `self.SpawnProjectile`
  (bind _particlesystem (`self.ParticleSystem`))
  ;[1 1 1] activate / deactive the emitter on fire
  (`ActorComponent.Activate` _particlesystem true)
  (`|ExecutionSequence`
    (:`then_0`
      (`KismetSystemLibrary.Delay` 2.1)
      (`ActorComponent.Deactivate` _particlesystem)
      (goto _label :!via `Close`))
    (:`then_1`
      (goto _label :!via `Open`))
    (:`then_2`
      (goto _label_2 :!via `Reset`))))

(fn `UserConstructionScript`
  (`parent.UserConstructionScript`))