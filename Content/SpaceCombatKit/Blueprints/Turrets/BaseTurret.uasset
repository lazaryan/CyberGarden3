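; Base turret, usually mounted on a BaseShip whose faction it inherits, that automatically engages targets and shatters into destructible meshes on death.
; A looping timer sphere-traces for interface-implementing targets, filtered by turret type and faction, then picks a visible one.
; Tick leads the target by velocity, rotating body yaw and barrel pitch in turret-local space, or returns to rest.
; When aligned, it fires server-spawned projectiles, cycling barrels and muzzle sockets with spread and recoil.
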(event `self.ReceiveAnyDamage`
  (params (Damage :type "Float (single-precision)") (DamageType :type "DamageType Object Reference") (InstigatedBy :type "Controller Object Reference") (DamageCauser :type "Actor Object Reference"))
  ;[1 1 1] Damage
  (if (`self.TakeDamage`)
    (bind _output_get (set `self.Health` (- (`self.Health`) Damage)))
    (if (<= _output_get 0.0)
      (`/Engine/EditorBlueprintResources/StandardMacros.DoOnce` false
        (:`Completed`
          (`self.DeathSequence`))))))

(event `self.ReceiveBeginPlay`
  ;[1 1 1] Begin play - set variables and start targetting timer
  (if (`|EnumEquality` (`self.Faction`) "NewEnumerator0")
    (cast `/Game/SpaceCombatKit/Blueprints/Ships/BaseClasses/BaseShip` (`self.GetParentActor`)
      (:`then`
        (`self.GetAndSetFaction`))
      (:`CastFailed`
        _)))
  (set `self.Health` (`self.MaxHealth`))
  (`KismetArrayLibrary.Array_Resize` (`self.CurrentBarrelMuzzleIndex`) (`KismetArrayLibrary.Array_Length` (`self.BarrelsToFireFrom`)))
  (`KismetSystemLibrary.K2_SetTimerDelegate` (delegate `CheckForTargets`) (+ (`self.SearchForTargetsPulseRate`) (`KismetMathLibrary.RandomFloatInRange` -0.1 0.1)) true)
  (`self.CheckForTargets`)
  (`self.UpdateObjectiveMarkerColour` (`self.HasObjectiveMarker`)))

(event `CheckForTargets`
  ;[1 1 1] Check for targets - if we don't have a primary target, run the targetting function to find one - based on our turret type
  (`/Engine/EditorBlueprintResources/StandardMacros.Gate` false :!label _label
    (:`Exit`
      (`/Engine/EditorBlueprintResources/StandardMacros.IsValid` (`self.PrimaryTarget`)
        (:`Is Not Valid`
          (`self.Targetting` (`self.TurretType`)))))))

(event `DeathSequence`
  ;[1 1 1] Death Sequence - close gates and replace with destructible
  (`|ExecutionSequence`
    (:`then_0`
      (goto _label_2 :!via `Close`))
    (:`then_1`
      (goto _label :!via `Close`))
    (:`then_2`
      (`self.ReplaceWithDestructible`))))

(event `self.ReceiveTick`
  (params (DeltaSeconds :type "Float (single-precision)"))
  (`/Engine/EditorBlueprintResources/StandardMacros.Gate` false :!label _label_2
    (:`Exit`
      (`/Engine/EditorBlueprintResources/StandardMacros.IsValid` (`self.PrimaryTarget`)
        (:`Is Valid`
          (`|ExecutionSequence`
            (:`then_0`
              ;[1 1 1] Have-Target Sequence
              (`|ExecutionSequence`
                (:`then_0`
                  ;[1 1 1] If we have a primary target, check if we can see it. If we can't, clear the primary target., if not anti-capital
                  (bind _cansee (`self.SightTraceActor` (`self.PrimaryTarget`)))
                  (if _cansee
                    _
                    (elif (`|EnumInequality` (`self.TurretType`) "NewEnumerator1")
                      (set `self.PrimaryTarget` null))))
                (:`then_1`
                  ;[1 1 1] If we have a primary target, get it's aim at location, and aim at it.
                  (`self.GetTargetLocation` (`self.TurretType`))
                  (`self.AimAtTarget`))
                (:`then_2`
                  ;[1 1 1] Check if we're aiming at our primary target and can see it. If so, call fire sequence
                  (bind _canfire (`self.CheckIfCanFire` (`self.AimingErrorTolerance`)))
                  (if _canfire
                    (`self.FireSequence`)))
                (:`then_3`
                  ;[1 1 1] Adjust barrels relative location towards default for recoil
                  (`self.RecoilInterp` (`self.RecoilInterpSpeed`)))))
            (:`then_1`
              ;[1 1 1] Closes and opens gates once, resetting when losing/acquiring target
              (`/Engine/EditorBlueprintResources/StandardMacros.DoOnce` false :!label _label_3
                (:`Completed`
                  (`|ExecutionSequence`
                    (:`then_0`
                      (goto _label_4 :!via `Open`))
                    (:`then_1`
                      (goto _label_5 :!via `Reset`))))))))
        (:`Is Not Valid`
          ;[1 1 1] When no target, rotate turret components towards zero rotation. Close this gate when reached
          (`|ExecutionSequence`
            (:`then_0`
              (`/Engine/EditorBlueprintResources/StandardMacros.Gate` true :!label _label_4
                (:`Exit`
                  (`self.InterpTurretRotationsToDefault` ; Macro that interps turret rotations
                    (:`Completed`
                      (goto _label_4 :!via `Close`))))))
            (:`then_1`
              (`/Engine/EditorBlueprintResources/StandardMacros.DoOnce` false :!label _label_5
                (:`Completed`
                  (goto _label_3 :!via `Reset`))))))))))

(event `FireSequence`
  (bind _currentbarrelindex (`self.CurrentBarrelIndex`))
  ;[1 1 1] Fire Sequence
  ;;[1 1 1] If we can fire, set can't fire, and fire a projectile from the current barrel index
  (if (`self.CanFire`)
    (set `self.CanFire` false)
    (`/Engine/EditorBlueprintResources/ActorMacros.Switch Has Authority`
      (:`Authority`
        (`self.FireFromBarrel` (`self.Projectile`) (`|GetArrayItem` (`self.BarrelsToFireFrom`) _currentbarrelindex) _currentbarrelindex (`self.ProjectileScale`)))
      (:`Remote`
        (`self.Server_FireFromBarrel`)))
    ;;[1 1 1] Increases barrel index if we can, if not, set it to 0
    (if (`KismetArrayLibrary.Array_IsValidIndex` (`self.BarrelsToFireFrom`) (+ (`self.CurrentBarrelIndex`) 1))
      (set `self.CurrentBarrelIndex` (+ (`self.CurrentBarrelIndex`) 1))
      (else
        (set `self.CurrentBarrelIndex` 0)))
    ;;[1 1 1] Delays by our attack speed until we can fire again
    (`KismetSystemLibrary.Delay` (/ (`self.AttackSpeed`) (`KismetMathLibrary.Conv_IntToDouble` (`KismetArrayLibrary.Array_Length` (`self.BarrelsToFireFrom`)))))
    (set `self.CanFire` true)))

(event `Server_FireFromBarrel`
  (bind _currentbarrelindex (`self.CurrentBarrelIndex`))
  ;[1 1 1] Server - Call fire from barrel
  (`self.FireFromBarrel` (`self.Projectile`) (`|GetArrayItem` (`self.BarrelsToFireFrom`) _currentbarrelindex) _currentbarrelindex 0.0))

(event `FireFromBarrel`
  (params (ProjectileToSpawn :type "/Game/SpaceCombatKit/Blueprints/Projectiles/BaseProjectile Class Reference") (BarrelToFireFrom :type "SceneComponent Object Reference") (BarrelIndex :type Integer) (Scale :type "Float (double-precision)" :default 1.0))
  ;[1 1 1] Fires a projectile from the supplied barrel
  (bind _socketname (`self.GetSocketToFireFrom` BarrelToFireFrom BarrelIndex)) ; Can't be pure as it updates the muzzle index
  (bind (_returnvalue_location _returnvalue_rotation) (`KismetMathLibrary.BreakTransform` (`SceneComponent.GetSocketTransform` BarrelToFireFrom _socketname "RTS_World")))
  (bind _returnvalue (`|SpawnActorFromClass` ProjectileToSpawn (`KismetMathLibrary.MakeTransform` _returnvalue_location (`self.CalculateSpread` _returnvalue_rotation) (`KismetMathLibrary.Conv_DoubleToVector` Scale)) "Undefined" "OverrideRootScale" self (`self.ProjectileSpeed`) (`self.ProjectileDamage`) (`self.ProjectileImpulseStrength`) (cast `Pawn` (`self.GetParentActor`) :!pure true)))
  (`SceneComponent.K2_AddLocalOffset` BarrelToFireFrom (`KismetMathLibrary.MakeVector` (`self.BarrelRecoil`)) false false)
  (`GameplayStatics.PlaySoundAtLocation` (`self.FireSound`) _returnvalue_location (struct) 1.0 1.0 0.0 "/Game/SpaceCombatKit/Sounds/Weapons/WeaponsFireAttenuation.WeaponsFireAttenuation")
  (bind _asproj_beam (cast `/Game/SpaceCombatKit/Blueprints/Projectiles/Proj_Beam` _returnvalue))
  (set `/Game/SpaceCombatKit/Blueprints/Projectiles/Proj_Beam.TurretFiredFrom` self _asproj_beam)
  (set `/Game/SpaceCombatKit/Blueprints/Projectiles/Proj_Beam.BarrelFiredFrom` BarrelToFireFrom _asproj_beam)
  (set `/Game/SpaceCombatKit/Blueprints/Projectiles/Proj_Beam.SocketNameFiredFrom` _socketname _asproj_beam))

(fn `AimAtTarget`
  ;[1 1 1] Rotates the turret components to face TargetLocation
  (`self.RotateTurretComponents` (`self.BodyMesh`) (`self.Barrel1Mesh`) (`self.GetTransformedRotationToTarget` (`self.GetTransform`) (`self.TargetLocation`) (`self.Barrel1Mesh`) "Muzzle")))

(fn `AimPredict`
  (returns (PredictedAimLocation :type "Vector Structure"))
  (bind _primarytarget (`self.PrimaryTarget`))
  (bind _returnvalue (/ (`KismetMathLibrary.VSize` (- (`self.K2_GetActorLocation` (`self.PrimaryTarget`)) (`SceneComponent.K2_GetComponentLocation` (`self.Barrel1Mesh`)))) (`self.ProjectileSpeed`)))
  (bind _asbase_ship (cast `/Game/SpaceCombatKit/Blueprints/Ships/BaseClasses/BaseShip` _primarytarget)
    (:`then`
      ;[1 1 1] if the target is a baseship, call GetShipVelocity instead of velocity
      (return (+ (`self.K2_GetActorLocation` _asbase_ship) (* (`/Game/SpaceCombatKit/Blueprints/Ships/BaseClasses/BaseShip.GetShipVelocity` _asbase_ship) _returnvalue))))
    (:`CastFailed`
      (return (+ (`self.K2_GetActorLocation` _primarytarget) (* (`self.GetVelocity` _primarytarget) _returnvalue))))))

(fn `CalculateSpread`
  (params (InRotation :type "Rotator Structure"))
  (returns (OutRotation :type "Rotator Structure"))
  (bind _spread_negative_ (`self.Spread(Negative)`))
  (bind _spread_negative__2 (`self.Spread(Negative)`))
  (bind _spread_negative__3 (`self.Spread(Negative)`))
  ;[1 1 1] Adds random spread based on spread value
  (return (`KismetMathLibrary.MakeRotator` (+ InRotation_Roll (`KismetMathLibrary.RandomFloatInRange` _spread_negative_ (`KismetMathLibrary.Abs` _spread_negative_))) (+ InRotation_Pitch (`KismetMathLibrary.RandomFloatInRange` _spread_negative__2 (`KismetMathLibrary.Abs` _spread_negative__2))) (+ InRotation_Yaw (`KismetMathLibrary.RandomFloatInRange` _spread_negative__3 (`KismetMathLibrary.Abs` _spread_negative__3))))))

(fn `CheckIfCanFire`
  (params (RotationErrorTolerance :type "Float (double-precision)"))
  (returns (CanFire :type Boolean))
  (bind (_relativerotation_roll _relativerotation_pitch) (`KismetMathLibrary.BreakRotator` (`SceneComponent.RelativeRotation` (`self.Barrel1Mesh`))))
  ;[1 1 1] Checks if we can see the actor
  (bind _cansee (`self.SightTraceActor` (`self.PrimaryTarget`)))
  ;[1 1 1] Returns whether or not we can fire
  (if (and (`KismetMathLibrary.NearlyEqual_FloatFloat` _relativerotation_pitch (.pitch (`self.GetTransformedRotationToTarget` (`self.GetTransform`) (`self.TargetLocation`) (`self.Barrel1Mesh`) "Muzzle")) RotationErrorTolerance) (`KismetMathLibrary.NearlyEqual_FloatFloat` (.yaw (`SceneComponent.RelativeRotation` (`self.BodyMesh`))) (.yaw (`self.GetTransformedRotationToTarget` (`self.GetTransform`) (`self.TargetLocation`) (`self.Barrel1Mesh`) "Muzzle")) RotationErrorTolerance) _cansee)
    (return true)
    (else
      (return false))))

(fn `GetAndSetFaction`
  ;[1 1 1] Get's the parent actors faction and sets ours to it
  (set `self.Faction` (`/Game/SpaceCombatKit/Blueprints/Ships/BaseClasses/BaseShip.Faction` (cast `/Game/SpaceCombatKit/Blueprints/Ships/BaseClasses/BaseShip` (`self.GetParentActor`) :!pure true))))

(fn `GetAnyTarget`
  (bind _returnvalue (`self.K2_GetActorLocation`))
  ;[1 1 1] Checks if we have and can see our primary target. If we can, do nothing. If we can't, clear primary target and check for a new one
  (`/Engine/EditorBlueprintResources/StandardMacros.IsValid` (`self.PrimaryTarget`)
    (:`Is Valid`
      (bind _cansee (`self.SightTraceActor` (`self.PrimaryTarget`)))
      (if (not _cansee)
        (set `self.PrimaryTarget` null)))
    (:`Is Not Valid`
      ;[1 1 1] Performs a sphere trace around the actor searching for targets that implement "Interface_TargetableByTurrets"
      (bind _outhits (`KismetSystemLibrary.SphereTraceMulti` _returnvalue (+ _returnvalue (0.0 0.0 10.0)) (`self.SearchRadius`) "TraceTypeQuery1" false (`|MakeArray` (`self.GetParentActor`))))
      (for _array_element _outhits
        (bind (_bblockinghit _binitialoverlap _time _location _impactpoint _normal _impactnormal _physmat _hitactor) (`GameplayStatics.BreakHitResult` _array_element))
        (if (`KismetSystemLibrary.DoesImplementInterface` _hitactor "/Game/SpaceCombatKit/Blueprints/Turrets/Interfaces/Interf_TurretTarget.Interf_TurretTarget_C")
          (bind _asbase_ship (cast `/Game/SpaceCombatKit/Blueprints/Ships/BaseClasses/BaseShip` _hitactor)
            (:`then`
              (if (`|EnumInequality` (`/Game/SpaceCombatKit/Blueprints/Ships/BaseClasses/BaseShip.Faction` _asbase_ship) (`self.Faction`))
                (`KismetArrayLibrary.Array_AddUnique` (`self.Targets`) _hitactor)))
            (:`CastFailed`
              (`KismetArrayLibrary.Array_AddUnique` (`self.Targets`) _hitactor))))))))

(fn `GetCapitalTarget`
  (bind _returnvalue (`self.K2_GetActorLocation`))
  ;[1 1 1] Checks if we have and can see our primary target. If we can, do nothing. If we can't, clear primary target and check for a new one
  (`/Engine/EditorBlueprintResources/StandardMacros.IsValid` (`self.PrimaryTarget`)
    (:`Is Valid`
      (bind _cansee (`self.SightTraceActor` (`self.PrimaryTarget`)))
      (if (not _cansee)
        (set `self.PrimaryTarget` null)))
    (:`Is Not Valid`
      ;[1 1 1] Performs a sphere trace around the actor searching for targets that implement "Interface_TargetableByTurrets"
      (bind _outhits (`KismetSystemLibrary.SphereTraceMulti` _returnvalue (+ _returnvalue (0.0 0.0 10.0)) (`self.SearchRadius`) "TraceTypeQuery1" false (`|MakeArray` (`self.GetParentActor`))))
      (for _array_element _outhits
        (bind (_bblockinghit _binitialoverlap _time _location _impactpoint _normal _impactnormal _physmat _hitactor) (`GameplayStatics.BreakHitResult` _array_element))
        (if (`KismetSystemLibrary.DoesImplementInterface` _hitactor "/Game/SpaceCombatKit/Blueprints/Turrets/Interfaces/Interf_TurretTarget.Interf_TurretTarget_C")
          (bind _asbase_ship (cast `/Game/SpaceCombatKit/Blueprints/Ships/BaseClasses/BaseShip` _hitactor)
            (:`then`
              (bind _iscapital (`/Game/SpaceCombatKit/Blueprints/Ships/BaseClasses/BaseShip.GetIsCapital` _asbase_ship))
              (if (and _iscapital (`|EnumInequality` (`/Game/SpaceCombatKit/Blueprints/Ships/BaseClasses/BaseShip.Faction` _asbase_ship) (`self.Faction`)))
                (`KismetArrayLibrary.Array_AddUnique` (`self.Targets`) _hitactor)))
            (:`CastFailed`
              (`KismetArrayLibrary.Array_AddUnique` (`self.Targets`) _hitactor))))))))

(fn `GetFighterTarget`
  (bind _returnvalue (`self.K2_GetActorLocation`))
  ;[1 1 1] Checks if we have and can see our primary target. If we can, do nothing. If we can't, clear primary target and check for a new one
  (`/Engine/EditorBlueprintResources/StandardMacros.IsValid` (`self.PrimaryTarget`)
    (:`Is Valid`
      (bind _cansee (`self.SightTraceActor` (`self.PrimaryTarget`)))
      (if (not _cansee)
        (set `self.PrimaryTarget` null)))
    (:`Is Not Valid`
      ;[1 1 1] Performs a sphere trace around the actor searching for targets that implement "Interface_TargetableByTurrets"
      (bind _outhits (`KismetSystemLibrary.SphereTraceMulti` _returnvalue (+ _returnvalue (0.0 0.0 10.0)) (`self.SearchRadius`) "TraceTypeQuery1" false (`|MakeArray` (`self.GetParentActor`))))
      (for _array_element _outhits
        (bind (_bblockinghit _binitialoverlap _time _location _impactpoint _normal _impactnormal _physmat _hitactor) (`GameplayStatics.BreakHitResult` _array_element))
        (if (`KismetSystemLibrary.DoesImplementInterface` _hitactor "/Game/SpaceCombatKit/Blueprints/Turrets/Interfaces/Interf_TurretTarget.Interf_TurretTarget_C")
          (bind _asbase_ship (cast `/Game/SpaceCombatKit/Blueprints/Ships/BaseClasses/BaseShip` _hitactor)
            (:`then`
              (bind _isfighter (`/Game/SpaceCombatKit/Blueprints/Ships/BaseClasses/BaseShip.GetIsFighter` _asbase_ship))
              (if (and _isfighter (`|EnumInequality` (`/Game/SpaceCombatKit/Blueprints/Ships/BaseClasses/BaseShip.Faction` _asbase_ship) (`self.Faction`)))
                (`KismetArrayLibrary.Array_AddUnique` (`self.Targets`) _hitactor)))
            (:`CastFailed`
              (`KismetArrayLibrary.Array_AddUnique` (`self.Targets`) _hitactor))))))))

(fn `GetSocketToFireFrom`
  (params (SceneComponent :type "SceneComponent Object Reference") (BarrelIndex :type Integer))
  (returns (SocketName :type Name))
  (locals (TempSocketName :type Name))
  (bind _returnvalue (`SceneComponent.GetAllSocketNames` SceneComponent))
  (bind _returnvalue_2 (`SceneComponent.GetAllSocketNames` SceneComponent))
  (bind _currentbarrelmuzzleindex (`self.CurrentBarrelMuzzleIndex`))
  (bind _returnvalue_3 (`KismetArrayLibrary.Array_LastIndex` _returnvalue))
  (if (> _returnvalue_3 0)
    (set `local.TempSocketName` (`|GetArrayItem` _returnvalue_2 (`|GetArrayItem` (`self.CurrentBarrelMuzzleIndex`) BarrelIndex)))
    ;[1 1 1] Checks if we can increase the barrel muzzle index
    (if (`KismetArrayLibrary.Array_IsValidIndex` _returnvalue_2 (+ (`|GetArrayItem` (`self.CurrentBarrelMuzzleIndex`) BarrelIndex) 1))
      ;[1 1 1] Increase barrle muzzle index and get that socket
      (`KismetArrayLibrary.Array_Set` _currentbarrelmuzzleindex BarrelIndex (+ (`|GetArrayItem` _currentbarrelmuzzleindex BarrelIndex) 1))
      (return (`local.TempSocketName`))
      (else
        ;[1 1 1] Set current barrel muzzle index to 0 and get that socket
        (`KismetArrayLibrary.Array_Set` (`self.CurrentBarrelMuzzleIndex`) BarrelIndex)
        (return (`local.TempSocketName`))))
    (else
      ;[1 1 1] Get the only socket if there isn't more than one
      (return (`|GetArrayItem` _returnvalue _returnvalue_3)))))

(fn `GetTargetLocation`
  (params (Selection :type "/Game/SpaceCombatKit/Blueprints/Turrets/E_TurretType Enum" :default "NewEnumerator0"))
  (`/Engine/EditorBlueprintResources/StandardMacros.IsValid` (`self.PrimaryTarget`)
    (:`Is Valid`
      (switch `/Game/SpaceCombatKit/Blueprints/Turrets/E_TurretType` Selection
        (:`NewEnumerator0`
          _)
        (:`NewEnumerator1`
          _)
        (:`NewEnumerator2`
          _)
        (:`NewEnumerator3`
          _))
      ;[1 1 1] Gets the fighter location and it's velocity - sets that as the target location
      (set `self.TargetLocation` (+ (`self.AimPredict`) (`self.TargetBoundingBoxOffset`))))))

(fn `GetTransformedRotationToTarget`
  (params (TransformOfBase :type "Transform Structure (by ref)") (TargetPosition :type "Vector Structure") (BarrelMesh :type "SceneComponent Object Reference") (SocketMeshIsMountedOn :type Name))
  (returns (Rotation :type "Rotator Structure"))
  ;[1 1 1] Gets the parents transform base, and gets the inverse transform direction of the barrels socket location, so that we can be rotated in any direction to face our target. Returns as a rotation we'll interp to
  (return (`KismetMathLibrary.MakeRotFromX` (`KismetMathLibrary.InverseTransformDirection` TransformOfBase (- TargetPosition (`SceneComponent.GetSocketLocation` BarrelMesh SocketMeshIsMountedOn))))))

(fn `RecoilInterp`
  (params (InterpSpeed :type "Float (double-precision)"))
  ;[1 1 1] For each barrel, interp their relative location to 0 so they return to firing position
  (for _array_element (`self.BarrelsToFireFrom`)
    (`SceneComponent.K2_SetRelativeLocation` _array_element (`KismetMathLibrary.VInterpTo` (`SceneComponent.RelativeLocation` _array_element) (0.0 0.0 0.0) (`GameplayStatics.GetWorldDeltaSeconds`) InterpSpeed) false false)))

(fn `ReplaceWithDestructible`
  (locals (BodyDM :type "DestructibleComponent Object Reference") (BarrelDM :type "DestructibleComponent Object Reference"))
  (bind _bodydm (`local.BodyDM`))
  (bind _barreldm (`local.BarrelDM`))
  (bind _children (`SceneComponent.GetChildrenComponents` (`self.Barrel1Mesh`) true))
  ;[1 1 1] Destroy all children of barrel1mesh - will replace barrels with static mesh DM
  (for _array_element _children
    (`ActorComponent.K2_DestroyComponent` _array_element))
  (for _array_element_2 _children
    (`ActorComponent.K2_DestroyComponent` _array_element_2))
  ;[1 1 1] For Barrel1Mesh and BodyMesh, add a destructible, set it's mesh to the relevant variable, and destroy the old mesh.
  (bind _returnvalue (`AddComponent|NODE_AddDestructibleComponent-1` :`RelativeTransform` (`SceneComponent.K2_GetComponentToWorld` (`self.Barrel1Mesh`))))
  (`ActorComponent.K2_DestroyComponent` (`self.Barrel1Mesh`))
  (`DestructibleComponent.SetDestructibleMesh` _returnvalue (`self.Barrel1DestructibleMesh`))
  (bind _output_get (set `local.BarrelDM` _returnvalue))
  (`PrimitiveComponent.SetEnableGravity` _output_get false)
  (bind _returnvalue_2 (`AddComponent|NODE_AddDestructibleComponent-2` :`RelativeTransform` (`SceneComponent.GetRelativeTransform` (`self.BodyMesh`))))
  (`DestructibleComponent.SetDestructibleMesh` _returnvalue_2 (`self.BodyDestructibleMesh`))
  (`ActorComponent.K2_DestroyComponent` (`self.BodyMesh`))
  (bind _output_get_2 (set `local.BodyDM` _returnvalue_2))
  (`PrimitiveComponent.SetEnableGravity` _output_get_2 false)
  ;[1 1 1] Explode the destructible meshes
  (`DestructibleComponent.ApplyRadiusDamage` _barreldm 500.0 (`SceneComponent.K2_GetComponentLocation` _barreldm) 500.0 500.0 false)
  (`DestructibleComponent.ApplyRadiusDamage` _bodydm 500.0 (`SceneComponent.K2_GetComponentLocation` _bodydm) 500.0 500.0 false)
  ;[1 1 1] Spawn death particle
  (bind _returnvalue_3 (`GameplayStatics.SpawnEmitterAtLocation` (`self.DeathParticle`) (`SceneComponent.K2_GetComponentLocation` (`local.BarrelDM`))))
  (`SceneComponent.SetWorldScale3D` _returnvalue_3 (`self.GetActorScale3D`))
  ;[1 1 1] Set Life Span
  (`self.SetLifeSpan` 7.0))

(fn `RotateTurretComponents`
  (params (BodyMesh :type "SceneComponent Object Reference") (Barrel1Mesh :type "SceneComponent Object Reference") (TargetRotation :type "Rotator Structure"))
  (bind (_relativerotation_roll _relativerotation_pitch) (`KismetMathLibrary.BreakRotator` (`SceneComponent.RelativeRotation` Barrel1Mesh)))
  (bind (_relativerotation_roll_2 _relativerotation_pitch_2 _relativerotation_yaw) (`KismetMathLibrary.BreakRotator` (`SceneComponent.RelativeRotation` BodyMesh)))
  (`|ExecutionSequence`
    (:`then_0`
      ;[1 1 1] Updates the body from it's current rotation to the desired rotation
      (`SceneComponent.K2_SetRelativeRotation` BodyMesh (`KismetMathLibrary.MakeRotator` 0.0 0.0 (`KismetMathLibrary.FInterpTo` _relativerotation_yaw (.yaw TargetRotation) (`GameplayStatics.GetWorldDeltaSeconds`) (`self.TurretYawRotationSpeed`))) false false))
    (:`then_1`
      ;[1 1 1] Updates the barrel from it's current rotation to the desired rotation
      (`SceneComponent.K2_SetRelativeRotation` Barrel1Mesh (`KismetMathLibrary.MakeRotator` 0.0 (`KismetMathLibrary.FInterpTo` _relativerotation_pitch (.pitch TargetRotation) (`GameplayStatics.GetWorldDeltaSeconds`) (`self.TurretPitchRotationSpeed`))) false false))))

(fn `SightTraceActor`
  (params (TargetActor :type "Actor Object Reference"))
  (returns (CanSee :type Boolean))
  ;[1 1 1] Line traces the target to see if we can see it
  (`/Engine/EditorBlueprintResources/StandardMacros.IsValid` TargetActor
    (:`Is Valid`
      (bind _outhit (`KismetSystemLibrary.LineTraceSingle` (`SceneComponent.K2_GetComponentLocation` (`self.Barrel1Mesh`)) (`self.K2_GetActorLocation` TargetActor) "TraceTypeQuery1"))
      (return (== (`.HitActor` (`GameplayStatics.BreakHitResult` _outhit)) TargetActor)))))

(fn `SortTargetsVisibilityAndDistance`
  (locals (ClosestDistanceCheck :type "Float (double-precision)" :default 50000.0) (TempPrimaryTarget :type "Actor Object Reference"))
  ;[1 1 1] Clears the local variables so the data will be fresh
  (set `local.ClosestDistanceCheck` 50000.0)
  (set `local.TempPrimaryTarget` null)
  ;[1 1 1] For each target, checks if we can see it. If we can, checks if it's closer than the last target we could see. If it is, set it to the temporary primary target
  (for _array_element (`self.Targets`)
    (bind _cansee (`self.SightTraceActor` _array_element))
    (if _cansee
      (bind _returnvalue (`self.GetDistanceTo` _array_element))
      (if (and (< _returnvalue (`local.ClosestDistanceCheck`)) (< _returnvalue (* (`self.SearchRadius`) 2.0)))
        (set `local.ClosestDistanceCheck` 0.0)
        (set `local.TempPrimaryTarget` _array_element))))
  ;[1 1 1] Sets the primary target to the temporary primary target
  (`/Engine/EditorBlueprintResources/StandardMacros.IsValid` (`local.TempPrimaryTarget`)
    (:`Is Valid`
      (set `self.PrimaryTarget` (`local.TempPrimaryTarget`)))))

(fn `Targetting`
  (params (TurretType :type "/Game/SpaceCombatKit/Blueprints/Turrets/E_TurretType Enum" :default "NewEnumerator0"))
  ;[1 1 1] Runs the relevant "get X target" function based on our turret type
  (switch `/Game/SpaceCombatKit/Blueprints/Turrets/E_TurretType` TurretType
    (:`NewEnumerator0`
      (`self.GetFighterTarget`))
    (:`NewEnumerator1`
      (`self.GetCapitalTarget`))
    (:`NewEnumerator2`
      (`self.GetAnyTarget`)))
  ;[1 1 1] Sorts all found targets
  (`self.SortTargetsVisibilityAndDistance`))

(fn `UpdateObjectiveMarkerColour`
  (params (HasObjectiveMarker :type Boolean))
  (bind _objectivemarkercomp (`self.ObjectiveMarkerComp`))
  (bind _faction (`self.Faction`))
  ;[1 1 1] Sets the colour of the objective targetting marker billboard based on faction. Sets the owner for Owner No See. Destroy if HasObjectiveMarker false
  (if HasObjectiveMarker
    (bind _asbp_objective_marker (cast `/Game/SpaceCombatKit/Blueprints/Components/BP_ObjectiveMarker` (`ChildActorComponent.ChildActor` _objectivemarkercomp)))
    (`/Game/SpaceCombatKit/Blueprints/Components/BP_ObjectiveMarker.UpdateColor` _asbp_objective_marker (select `/Game/SpaceCombatKit/Blueprints/Game/E_FactionsEnum` _faction :`NewEnumerator0` 0.2 :!type "Float (single-precision)") (select `/Game/SpaceCombatKit/Blueprints/Game/E_FactionsEnum` _faction :`NewEnumerator0` 0.2 :`NewEnumerator2` 1.0 :!type "Float (single-precision)") (select `/Game/SpaceCombatKit/Blueprints/Game/E_FactionsEnum` _faction :`NewEnumerator0` 0.2 :!type "Float (single-precision)"))
    (`self.SetOwner` _asbp_objective_marker self)
    (else
      (`ActorComponent.K2_DestroyComponent` _objectivemarkercomp))))

(fn `UserConstructionScript`
  ;[1 1 1] Sets the barrels to to fire projectiles from
  (set `self.BarrelsToFireFrom` (`|MakeArray` (`self.Barrel1Mesh`) :!type "SceneComponent Object Reference")))