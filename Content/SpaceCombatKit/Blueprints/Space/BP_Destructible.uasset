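; BP_Destructible is a space combat destructible that blows itself apart as soon as it spawns.
; BeginPlay applies heavy radius damage to the configurable mesh, then clears the Explosions flag after a set lifetime.
; While that flag is set, Tick uses a short random Delay to stagger explosion emitters at random mesh sockets, each scaled randomly relative to the destructible's size.
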(event `self.ReceiveBeginPlay`
  (bind _destructible (`self.Destructible`))
  ;[1 1 1] On begin play, apply damage so that the destructible explodes.
  (`DestructibleComponent.ApplyRadiusDamage` _destructible 150000.0 (`SceneComponent.K2_GetComponentLocation` _destructible) (`self.DamageRadius`) (`self.ImpulseStrength`) true)
  (`KismetSystemLibrary.Delay` (`self.ExplosionLifeTIme`))
  (set `self.Explosions` false))

(event `self.ReceiveTick`
  (params (DeltaSeconds :type "Float (single-precision)"))
  (bind _returnvalue (`SceneComponent.GetAllSocketNames` (`self.Destructible`)))
  (if (`self.Explosions`)
    (`KismetSystemLibrary.Delay` (`KismetMathLibrary.RandomFloatInRange` 0.075 0.15))
    (`self.SpawnExplosion` (`SceneComponent.GetSocketLocation` (`self.Destructible`) (`|GetArrayItem` _returnvalue (`KismetMathLibrary.RandomIntegerInRange` 0 (`KismetArrayLibrary.Array_LastIndex` _returnvalue)))))))

(fn `SpawnExplosion`
  (params (Location :type "Vector Structure"))
  (bind _returnvalue (`GameplayStatics.SpawnEmitterAtLocation` "/Game/SpaceCombatKit/Particles/StarterContent/Particles/P_Explosion.P_Explosion" Location (struct)))
  (`SceneComponent.SetWorldScale3D` _returnvalue (* (`SceneComponent.RelativeScale3D` (`self.Destructible`)) (`KismetMathLibrary.RandomFloatInRange` 0.05 0.1))))

(fn `UserConstructionScript`
  (`DestructibleComponent.SetDestructibleMesh` (`self.Destructible`) (`self.DestructibleMesh`)))