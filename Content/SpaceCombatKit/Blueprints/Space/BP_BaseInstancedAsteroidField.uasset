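; Base asteroid field for the space combat kit that scatters instanced asteroids and can swap individual ones for destructibles.
; The construction script rebuilds one shadowless instanced mesh component per asteroid mesh, then adds randomly transformed instances within configurable distance and scale ranges.
; DetermineNearestAsteroid linearly searches all instances for the one closest to a hit location.
; ReplaceWithDestructible spawns a BP_Destructible at a given instance's transform and removes that instance.
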(fn `DetermineNearestAsteroid`
  (params (HitLocation :type "Vector Structure"))
  (returns (AsteroidToAffect :type Integer) (InstancedStaticMesh :type "InstancedStaticMeshComponent Object Reference") (ArrayIndex :type Integer))
  (set `self.BestDistanceToAsteroid` 500000.0) ; Variable used as the distance to the nearest asteroid for current iteration
  ;[1 1 1] For Each instanced static mesh in the asteroid field
  (for (_array_element _array_index) (`self.InstancedStaticMeshes`)
    ;[1 1 1] For each asteroid
    (for _index (range (+ (`InstancedStaticMeshComponent.GetInstanceCount` _array_element) 1))
      (bind _returnvalue (`KismetMathLibrary.VSize` (- (.location (`InstancedStaticMeshComponent.GetInstanceTransform` _array_element _index true)) HitLocation)))
      ;[1 1 1] If the distance to this asteroid is less than the best, set this one to the best. Set the instanced static mesh too
      (if (< _returnvalue (`self.BestDistanceToAsteroid`))
        (set `self.BestDistanceToAsteroid` _returnvalue)
        (set `self.AsteroidToDestroyIndex` _index)
        (set `self.InstancedComponentToAffect` _array_element))))
  ;[1 1 1] Return the best asteroid and it's instanced component
  (return (`self.AsteroidToDestroyIndex`) (`self.InstancedComponentToAffect`) _array_index))

(fn `ReplaceWithDestructible`
  (params (RoidToReplace :type Integer) (InstancedStaticMesh :type "InstancedStaticMeshComponent Object Reference") (DestructibleIndex :type Integer))
  (bind _outinstancetransform (`InstancedStaticMeshComponent.GetInstanceTransform` InstancedStaticMesh RoidToReplace true))
  ;[1 1 1] Gets the asteroid and replaces it with a destructable
  (`|SpawnActorFromClass` "/Game/SpaceCombatKit/Blueprints/Space/BP_Destructible.BP_Destructible_C" (`KismetMathLibrary.MakeTransform` (.location _outinstancetransform) (.rotation _outinstancetransform) (.scale _outinstancetransform)) "AlwaysSpawn" "OverrideRootScale" null (`|GetArrayItem` (`self.AsteroidDestructibleMeshes`) DestructibleIndex) 5000.0 5000.0 false 8.0 null)
  (`InstancedStaticMeshComponent.RemoveInstance` InstancedStaticMesh RoidToReplace))

(fn `UserConstructionScript`
  (bind _instancedstaticmeshes (`self.InstancedStaticMeshes`))
  (bind _instancedstaticmeshes_2 (`self.InstancedStaticMeshes`))
  (bind _asteroidmeshestouse (`self.AsteroidMeshesToUse`))
  ;[1 1 1] This clears the array so we're starting with a fresh slate and so instanced components don't stack up
  (for _array_element _instancedstaticmeshes
    (`ActorComponent.K2_DestroyComponent` _array_element))
  (`KismetArrayLibrary.Array_Clear` _instancedstaticmeshes)
  ;[1 1 1] For each static mesh in the array, add an instanced mesh component, and set it's static mesh
  (for (_ _array_index) _asteroidmeshestouse
    (bind _returnvalue (`AddComponent|NODE_AddInstancedStaticMeshComponent-0` :`RelativeTransform` (`KismetMathLibrary.MakeTransform` (0.0 0.0 0.0))))
    (`KismetArrayLibrary.Array_Add` (`self.InstancedStaticMeshes`) _returnvalue)
    (`StaticMeshComponent.SetStaticMesh` _returnvalue (`|GetArrayItem` _asteroidmeshestouse _array_index))
    (`PrimitiveComponent.SetCastShadow` _returnvalue false))
  ;[1 1 1] For every Total Roid, add an instanced roid with a random transform
  (for _ (range (+ (`self.TotalRoids`) 1))
    (`InstancedStaticMeshComponent.AddInstance` (`|GetArrayItem` _instancedstaticmeshes_2 (`KismetMathLibrary.RandomIntegerInRange` 0 (`KismetArrayLibrary.Array_LastIndex` _instancedstaticmeshes_2))) (`KismetMathLibrary.MakeTransform` (* (`KismetMathLibrary.RandomUnitVector`) (`KismetMathLibrary.MakeVector` (`KismetMathLibrary.RandomFloatInRange` (`self.MinDistanceXY`) (`self.MaxDistanceXY`)) (`KismetMathLibrary.RandomFloatInRange` (`self.MinDistanceXY`) (`self.MaxDistanceXY`)) (`KismetMathLibrary.RandomFloatInRange` (`self.MinDistanceZ`) (`self.MaxDistanceZ`)))) (`KismetMathLibrary.RandomRotator` false) (`KismetMathLibrary.Conv_DoubleToVector` (* (`KismetMathLibrary.RandomFloatInRange` (`self.MinScale`) (`self.MaxScale`)) (`self.ScaleMultiplier`)))))))