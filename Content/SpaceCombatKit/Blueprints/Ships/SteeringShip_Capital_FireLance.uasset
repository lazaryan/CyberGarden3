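; FireLance capital ship Blueprint, a steerable ship with three primary beam weapons and left and right fighter hangars with animated doors.
; Open and close events toggle per-side gates on Tick, which drive the OpenHang macro to interpolate door rotations.
; Fighters leaving the forcefield are unattached, and leaving a side's detection box closes their own hangar after a delay.
; The construction script skins the doors and registers the weapons.
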(event `self.ReceiveTick`
  (params (DeltaSeconds :type "Float (single-precision)"))
  ;[1 1 1] Tick Sequence
  (`parent.ReceiveTick` DeltaSeconds)
  (`|ExecutionSequence`
    (:`then_0`
      ;[1 1 1] Hangar Open/Close Sequences
      ;;[1 1 1] Left side
      (`/Engine/EditorBlueprintResources/StandardMacros.Gate` true :!label _label
        (:`Exit`
          (`self.OpenHang` (`self.HangarDoorLowerLeft`) (struct :`Roll` -90.0) (`self.HangarDoorUpperLeft`) (struct :`Roll` 90.0)
            (:`Complete`
              (goto _label :!via `Close`))))))
    (:`then_1`
      (`/Engine/EditorBlueprintResources/StandardMacros.Gate` true :!label _label_2
        (:`Exit`
          (`self.OpenHang` (`self.HangarDoorLowerLeft`) (struct) (`self.HangarDoorUpperLeft`)
            (:`Complete`
              (goto _label_2 :!via `Close`))))))
    (:`then_2`
      ;;[1 1 1] Right side
      (`/Engine/EditorBlueprintResources/StandardMacros.Gate` true :!label _label_3
        (:`Exit`
          (`self.OpenHang` (`self.HangarDoorLowerRight`) (struct :`Roll` 90.0) (`self.HangarDoorUpperRight`) (struct :`Roll` -90.0)
            (:`Complete`
              (goto _label_3 :!via `Close`))))))
    (:`then_3`
      (`/Engine/EditorBlueprintResources/StandardMacros.Gate` true :!label _label_4
        (:`Exit`
          (`self.OpenHang` (`self.HangarDoorLowerRight`) (struct) (`self.HangarDoorUpperRight`)
            (:`Complete`
              (goto _label_4 :!via `Close`))))))))

(event `self.OpenHangarIndex`
  (params (Index :type Integer))
  ;[1 1 1] Hangar Open/Close Sequences
  ;;[1 1 1] Left side
  (switch `int` Index
    (:`0`
      ;;[1 1 1] Right side
      (`|ExecutionSequence`
        (:`then_0`
          (goto _label_4 :!via `Close`))
        (:`then_1`
          (goto _label_3 :!via `Open`))))
    (:`1`
      (`|ExecutionSequence`
        (:`then_0`
          (goto _label_2 :!via `Close`))
        (:`then_1`
          (goto _label :!via `Open`))))))

(event `self.CloseHangarIndex`
  (params (Index :type Integer))
  ;[1 1 1] Hangar Open/Close Sequences
  ;;[1 1 1] Left side
  (switch `int` Index
    (:`0`
      ;;[1 1 1] Right side
      (`|ExecutionSequence`
        (:`then_0`
          (goto _label_3 :!via `Close`))
        (:`then_1`
          (goto _label_4 :!via `Open`))))
    (:`1`
      (`|ExecutionSequence`
        (:`then_0`
          (goto _label :!via `Close`))
        (:`then_1`
          (goto _label_2 :!via `Open`))))))

(event `self.HangarForceFields.OnComponentEndOverlap`
  (params (OverlappedComponent :type "PrimitiveComponent Object Reference") (OtherActor :type "Actor Object Reference") (OtherComp :type "PrimitiveComponent Object Reference") (OtherBodyIndex :type Integer))
  ;[1 1 1] When the forcefield ends overlap with a fighter, call Unattach Fighter to unlock it's controls, reset the hangar
  (bind _asbase_fighter (cast `/Game/SpaceCombatKit/Blueprints/Ships/BaseClasses/BaseFighter` OtherActor))
  (`self.UnattachFighter` _asbase_fighter))

(event `self.RightHangarLeaveDetect.OnComponentEndOverlap`
  (params (OverlappedComponent :type "PrimitiveComponent Object Reference") (OtherActor :type "Actor Object Reference") (OtherComp :type "PrimitiveComponent Object Reference") (OtherBodyIndex :type Integer))
  ;[1 1 1] If the box outside the RIGHT hangar ends overlap with the fighter who spawned in the RIGHT hangar, close that hangar
  (bind _asbase_fighter (cast `/Game/SpaceCombatKit/Blueprints/Ships/BaseClasses/BaseFighter` OtherActor))
  (if (== (`|GetArrayItem` (`self.StartHangarSockets`)) (`/Game/SpaceCombatKit/Blueprints/Ships/BaseClasses/BaseFighter.OwningHangarSocket` _asbase_fighter))
    (`KismetSystemLibrary.Delay` 1.0)
    (`self.CloseHangarIndex` 0)))

(event `self.LeftHangarLeaveDetect.OnComponentEndOverlap`
  (params (OverlappedComponent :type "PrimitiveComponent Object Reference") (OtherActor :type "Actor Object Reference") (OtherComp :type "PrimitiveComponent Object Reference") (OtherBodyIndex :type Integer))
  ;[1 1 1] If the box outside the LEFT hangar ends overlap with teh fighter who spawned in the LEFT hangar, close that hangar
  (bind _asbase_fighter (cast `/Game/SpaceCombatKit/Blueprints/Ships/BaseClasses/BaseFighter` OtherActor))
  (if (== (`|GetArrayItem` (`self.StartHangarSockets`) 1) (`/Game/SpaceCombatKit/Blueprints/Ships/BaseClasses/BaseFighter.OwningHangarSocket` _asbase_fighter))
    (`KismetSystemLibrary.Delay` 1.0)
    (`self.CloseHangarIndex` 1)))

(fn `DestructionEffects`)

(fn `UserConstructionScript`
  (`parent.UserConstructionScript`)
  ;[1 1 1] Sets the skins on the hangar doors
  (for _array_element (`|MakeArray` (`self.HangarDoorUpperRight`) (`self.HangarDoorUpperLeft`) (`self.HangarDoorLowerLeft`) (`self.HangarDoorLowerRight`) :!type "PrimitiveComponent Object Reference")
    (`self.SetSkin` _array_element (`self.GetSkinToUse`)))
  ;[1 1 1] Adds beam weapons to weapons array
  (`self.SetWeaponsArrays` (`|MakeArray` (`self.Beam1`) (`self.Beam2`) (`self.Beam3`)) (`|MakeArray` null :!type "ChildActorComponent Object Reference")))