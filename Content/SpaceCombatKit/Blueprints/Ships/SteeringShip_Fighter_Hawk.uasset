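; Hawk fighter ship Blueprint that extends a parent fighter class, with child-actor weapons assigned to primary and secondary arrays in the construction script.
; Tick runs parent logic only when a PlayerController possesses the ship.
; Otherwise, while controls are locked, it flies forward at the steering component's max speed to exit the hangar, unlocking 2000 units from its owning capital ship.
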(event `self.ReceiveBeginPlay`
  (`parent.ReceiveBeginPlay`))

(event `self.ReceiveTick`
  (params (DeltaSeconds :type "Float (single-precision)"))
  (bind _bpc_steeringbehaviourcomponent (`self.BPC_SteeringBehaviourComponent`))
  (bind _maxspeed (`/Game/SpaceCombatKit/Blueprints/Components/BPC_SteeringBehaviourComponent.MaxSpeed` _bpc_steeringbehaviourcomponent))
  ;[1 1 1] Used to make ships fly out of the hanger on spawn if their controls are locked
  ;;[1 1 1] Quick and easy way to enable player controls from parent class (BaseFighter)
  (cast `PlayerController` (`self.GetController`)
    (:`then`
      (`parent.ReceiveTick` DeltaSeconds))
    (:`CastFailed`
      (if (`self.ControlsLocked`)
        (bind _output_get (set `MovementComponent.Velocity` (`/Game/SpaceCombatKit/Blueprints/Components/BPC_SteeringBehaviourComponent.TruncateVector` _bpc_steeringbehaviourcomponent (* (`self.GetActorForwardVector`) _maxspeed) _maxspeed) (`self.CharacterMovement`)))
        (set `/Game/SpaceCombatKit/Blueprints/Components/BPC_SteeringBehaviourComponent.Velocity` _output_get (`self.BPC_SteeringBehaviourComponent`))
        (if (>= (`KismetMathLibrary.VSize` (- (`self.K2_GetActorLocation` (`self.OwningCapital`)) (`self.K2_GetActorLocation`))) 2000.0)
          (set `self.ControlsLocked` false))))))

(event `self.ReceiveAnyDamage`
  (params (Damage :type "Float (single-precision)") (DamageType :type "DamageType Object Reference") (InstigatedBy :type "Controller Object Reference") (DamageCauser :type "Actor Object Reference"))
  (`parent.ReceiveAnyDamage` Damage DamageType InstigatedBy DamageCauser))

(fn `UserConstructionScript`
  (`parent.UserConstructionScript`)
  (`self.SetWeaponsArrays` (`|MakeArray` (`self.ChildActor_0`) (`self.ChildActor1`) (`self.ChildActor2`)) (`|MakeArray` (`self.ChildActor3`) (`self.ChildActor_1`))))