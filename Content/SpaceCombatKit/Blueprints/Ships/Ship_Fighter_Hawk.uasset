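; Hawk fighter ship Blueprint from Space Combat Kit that configures its weapon and engine effect components on top of an inherited parent ship class.
; The construction script registers a cannon and two miniguns as primary weapons, two missile launchers as secondary weapons, and four engine particle components.
; BeginPlay and Tick only call the parent, so no runtime behavior is added here.
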(event `self.ReceiveBeginPlay`
  (`parent.ReceiveBeginPlay`))

(event `self.ReceiveTick`
  (params (DeltaSeconds :type "Float (single-precision)"))
  (`parent.ReceiveTick` DeltaSeconds))

(fn `UserConstructionScript`
  (`parent.UserConstructionScript`)
  (`self.SetWeaponsArrays` (`|MakeArray` (`self.Cannon`) (`self.Minigun1`) (`self.Minigun2`)) (`|MakeArray` (`self.MissileLauncher1`) (`self.MissileLauncher2`)))
  (`self.SetEngineParticles` (`|MakeArray` (`self.EngineParticle1`) (`self.EngineParticle2`) (`self.EngineParticle3`) (`self.EngineParticle4`))))