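; Tracer bullet projectile for space combat that flies straight along its forward vector at a set speed.
; Each tick it line-traces the next step, ignoring its instigator, and moves only if nothing blocks.
; Hits damage ships and turrets, push non-capital ships (capitals are exempt to keep spline following intact), or swap the nearest instanced asteroid for a destructible.
; Any blocking hit spawns a scaled impact emitter and destroys the bullet.
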(event `self.ReceiveBeginPlay`
  ;[1 1 1] Begin play - set our velocity to forward vector * speed
  (set `self.Velocity` (* (`self.GetActorForwardVector`) (`self.Speed`))))

(event `HitTurret`
  (params (HitTurret :type "/Game/SpaceCombatKit/Blueprints/Turrets/BaseTurret Object Reference"))
  ;[1 1 1] Hit turret - apply damage
  (`GameplayStatics.ApplyDamage` HitTurret (`self.Damage`))
  (bind _returnvalue (`GameplayStatics.SpawnEmitterAtLocation` (`self.HitEmitter`) (`self.K2_GetActorLocation`)))
  (`SceneComponent.SetWorldScale3D` _returnvalue (0.1 0.1 0.1))
  (`self.K2_DestroyActor`))

(event `self.ReceiveTick`
  (params (DeltaSeconds :type "Float (single-precision)"))
  (bind _returnvalue (`self.K2_GetActorLocation`))
  (bind _returnvalue_2 (+ _returnvalue (* (`self.Velocity`) (`GameplayStatics.GetWorldDeltaSeconds`))))
  ;[1 1 1] Trace forward and check for hits
  (bind _outhit (`KismetSystemLibrary.LineTraceSingle` _returnvalue _returnvalue_2 "TraceTypeQuery2" true (`|MakeArray` (`self.Instigator`) :!type "Actor Object Reference")))
  (if (`GameplayStatics.BreakHitResult` _outhit)
    ;[1 1 1] Checks if we hit a ship - and if so call Hit Ship
    (bind _asbase_ship (cast `/Game/SpaceCombatKit/Blueprints/Ships/BaseClasses/BaseShip` (`.HitActor` (`GameplayStatics.BreakHitResult` _outhit)))
      (:`then`
        (`self.HitShip` _asbase_ship (`.Location` (`GameplayStatics.BreakHitResult` _outhit)) (`.ImpactNormal` (`GameplayStatics.BreakHitResult` _outhit))))
      (:`CastFailed`
        ;[1 1 1] HitTurret
        (bind _asbase_turret (cast `/Game/SpaceCombatKit/Blueprints/Turrets/BaseTurret` (`.HitActor` (`GameplayStatics.BreakHitResult` _outhit)))
          (:`then`
            (`self.HitTurret` _asbase_turret))
          (:`CastFailed`
            (bind _asbp_base_instanced_asteroid_field (cast `/Game/SpaceCombatKit/Blueprints/Space/BP_BaseInstancedAsteroidField` (`.HitActor` (`GameplayStatics.BreakHitResult` _outhit)))
              (:`then`
                (bind (_asteroidtoaffect _instancedstaticmesh _arrayindex) (`/Game/SpaceCombatKit/Blueprints/Space/BP_BaseInstancedAsteroidField.DetermineNearestAsteroid` _asbp_base_instanced_asteroid_field (`.Location` (`GameplayStatics.BreakHitResult` _outhit))))
                (`/Game/SpaceCombatKit/Blueprints/Space/BP_BaseInstancedAsteroidField.ReplaceWithDestructible` _asbp_base_instanced_asteroid_field _asteroidtoaffect _instancedstaticmesh _arrayindex))
              (:`CastFailed`
                _))
            ;[1 1 1] Hit something else
            (bind _returnvalue_3 (`GameplayStatics.SpawnEmitterAtLocation` (`self.HitEmitter`) (`self.K2_GetActorLocation`)))
            (`SceneComponent.SetWorldScale3D` _returnvalue_3 (/ (`SceneComponent.K2_GetComponentScale` (`self.ParticleSystem`)) 5.0))
            (`self.K2_DestroyActor`)))))
    (else
      ;[1 1 1] If we didn't hit anything, move forward
      (`self.K2_SetActorLocation` _returnvalue_2))))

(event `HitShip`
  (params (HitShip :type "/Game/SpaceCombatKit/Blueprints/Ships/BaseClasses/BaseShip Object Reference") (HitLocation :type "Vector Structure") (HitNormal :type "Vector Structure"))
  ;[1 1 1] Hit ship - apply damage and add impulse
  (`GameplayStatics.ApplyDamage` HitShip (`self.Damage`))
  (cast `/Game/SpaceCombatKit/Blueprints/Ships/BaseClasses/BaseCapital` HitShip ; Check if it's a capital
    (:`then`
      _)
    (:`CastFailed`
      (`/Engine/EditorBlueprintResources/StandardMacros.IsValid` HitShip
        (:`Is Valid`
          (`CharacterMovementComponent.AddImpulse` (`Character.CharacterMovement` HitShip) (* (* HitNormal (`self.ImpulseStrength`)) -1.0) false) ; Impulse applied to capitals breaks spline following. Plus, they're heavy and shouldn't be moved from a bullet
        )
        (:`Is Not Valid`
          _))))
  (bind _returnvalue (`GameplayStatics.SpawnEmitterAtLocation` (`self.HitEmitter`) (`self.K2_GetActorLocation`)))
  (`SceneComponent.SetWorldScale3D` _returnvalue (0.1 0.1 0.1))
  (`self.K2_DestroyActor`))

(fn `UserConstructionScript`
  (`parent.UserConstructionScript`))