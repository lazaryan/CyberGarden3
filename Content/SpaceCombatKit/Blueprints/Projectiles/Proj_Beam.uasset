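; Beam weapon projectile for space combat that damages ships and breaks up instanced asteroids.
; Each tick it traces forward and stretches the particle beam from the firing barrel socket to the hit or maximum range.
; After a distance-based travel delay, a timed gate repeats damage and explosions on ships, while asteroids are swapped for destructibles once.
; Color comes from an override or the instigator's faction, and the actor dies with its particle or barrel.
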(event `self.ReceiveBeginPlay`
  (bind _beamrgbcolor (`self.BeamRGBColor`))
  ;[1 1 1] On begin play, bind an event to destroy this projectile when the particle ends
  (add `ActorComponent.OnComponentDeactivated` (`self.ParticleSystem`) (delegate `DestroySelf`))
  ;[1 1 1] Set the beam color on begin play, based on either the set color, or factions if it's not set
  (`ParticleSystemComponent.SetVectorParameter` (`self.ParticleSystem`) "color" (select `bool` (!= _beamrgbcolor (0.0 0.0 0.0)) :`false` (select `/Game/SpaceCombatKit/Blueprints/Game/E_FactionsEnum` (`/Game/SpaceCombatKit/Blueprints/Ships/BaseClasses/BaseShip.Faction` (cast `/Game/SpaceCombatKit/Blueprints/Ships/BaseClasses/BaseShip` (`self.Instigator`) :!pure true)) :`NewEnumerator0` (1.0 1.0 50.0) :`NewEnumerator2` (1.0 50.0 1.0) :`NewEnumerator1` (50.0 1.0 1.0) :!type "Vector Structure") :`true` _beamrgbcolor)))

(event `DestroySelf`
  (params (Component :type "ActorComponent Object Reference"))
  ;[1 1 1] On begin play, bind an event to destroy this projectile when the particle ends
  (`self.K2_DestroyActor`))

(event `self.ReceiveTick`
  (params (DeltaSeconds :type "Float (single-precision)"))
  (bind _returnvalue (`self.K2_GetActorLocation`))
  (bind _particlesystem (`self.ParticleSystem`))
  (bind _barrelfiredfrom (`self.BarrelFiredFrom`))
  (bind _returnvalue_2 (+ _returnvalue (* (`self.GetActorForwardVector`) (`self.BeamLength`))))
  (`/Engine/EditorBlueprintResources/StandardMacros.IsValid` _barrelfiredfrom
    (:`Is Valid`
      ;[1 1 1] Trace forward. If he hit something, set that as the end of the beam emitter. If not, forward vector * distance
      (`|ExecutionSequence`
        (:`then_0`
          (bind (_outhit _returnvalue_3) (`KismetSystemLibrary.LineTraceSingle` _returnvalue _returnvalue_2 "TraceTypeQuery1"))
          (`ParticleSystemComponent.SetBeamSourcePoint` _particlesystem 0 (`SceneComponent.GetSocketLocation` _barrelfiredfrom (`self.SocketNameFiredFrom`)) 0)
          (bind _returnvalue_4 (select `bool` _returnvalue_3 :`false` _returnvalue_2 :`true` (`.Location` (`GameplayStatics.BreakHitResult` _outhit))))
          (`ParticleSystemComponent.SetBeamTargetPoint` _particlesystem 0 _returnvalue_4 0)
          (bind _returnvalue_5 (`KismetMathLibrary.VSize` (- _returnvalue _returnvalue_4)))
          (`ParticleSystemComponent.SetFloatParameter` _particlesystem "distance" _returnvalue_5)
          (`ParticleSystemComponent.SetFloatParameter` _particlesystem "taperscale" (`self.BeamWidth`))
          (bind _asbase_ship (cast `/Game/SpaceCombatKit/Blueprints/Ships/BaseClasses/BaseShip` (`.HitActor` (`GameplayStatics.BreakHitResult` _outhit)))
            (:`then`
              (bind _output_get (set `self.HitShip` _asbase_ship))
              (`|ExecutionSequence`
                (:`then_0`
                  (`/Engine/EditorBlueprintResources/StandardMacros.DoOnce` false
                    (:`Completed`
                      (bind _returnvalue_6 (/ _returnvalue_5 30000.0))
                      (`KismetSystemLibrary.Delay` _returnvalue_6) ; Delays until the beam hits the target
                      (set `self.DelayUntilSparks` 0.0)
                      (goto _label :!via `Open`))))
                (:`then_1`
                  (`KismetSystemLibrary.Delay` 1.5) ; Delays until the beam ends
                  (goto _label :!via `Close`))))
            (:`CastFailed`
              (bind _asbp_base_instanced_asteroid_field (cast `/Game/SpaceCombatKit/Blueprints/Space/BP_BaseInstancedAsteroidField` (`.HitActor` (`GameplayStatics.BreakHitResult` _outhit))))
              (`/Engine/EditorBlueprintResources/StandardMacros.DoOnce` false
                (:`Completed`
                  (`KismetSystemLibrary.Delay` _returnvalue_6) ; Delays until the beam hits the target
                  (`/Engine/EditorBlueprintResources/StandardMacros.IsValid` _asbp_base_instanced_asteroid_field
                    (:`Is Valid`
                      (bind (_asteroidtoaffect _instancedstaticmesh _arrayindex) (`/Game/SpaceCombatKit/Blueprints/Space/BP_BaseInstancedAsteroidField.DetermineNearestAsteroid` _asbp_base_instanced_asteroid_field (`.Location` (`GameplayStatics.BreakHitResult` _outhit))))
                      (`/Game/SpaceCombatKit/Blueprints/Space/BP_BaseInstancedAsteroidField.ReplaceWithDestructible` _asbp_base_instanced_asteroid_field _asteroidtoaffect _instancedstaticmesh _arrayindex))))))))
        (:`then_1`
          ;;[1 1 1] Spawns an explosion and does damage every X seconds while the emitter is still active
          (`/Engine/EditorBlueprintResources/StandardMacros.Gate` true :!label _label
            (:`Exit`
              (`KismetSystemLibrary.Delay` (`self.DelayUntilSparks`))
              (`/Engine/EditorBlueprintResources/StandardMacros.IsValid` _output_get
                (:`Is Valid`
                  (bind _returnvalue_7 (`GameplayStatics.SpawnEmitterAttached` "/Game/SpaceCombatKit/Particles/StarterContent/Particles/P_Explosion.P_Explosion" (`/Game/SpaceCombatKit/Blueprints/Ships/BaseClasses/BaseShip.ShipMesh` _output_get) "None" (`.Location` (`GameplayStatics.BreakHitResult` _outhit)) (`KismetMathLibrary.Conv_VectorToRotator` (`.Normal` (`GameplayStatics.BreakHitResult` _outhit))) "KeepWorldPosition"))
                  (`GameplayStatics.ApplyDamage` _output_get (`self.Damage`))
                  (`/Engine/EditorBlueprintResources/StandardMacros.IsValid` _returnvalue_7
                    (:`Is Valid`
                      (`SceneComponent.SetWorldScale3D` _returnvalue_7 (2.0 2.0 2.0))
                      (set `self.DelayUntilSparks` 0.1))))))))))
    (:`Is Not Valid`
      (`self.K2_DestroyActor`))))

(fn `UserConstructionScript`)