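; AI controller for 6DoF fighter ships that patrol, hunt enemy-faction targets and fire primary weapons when in range.
; A timed sphere-overlap scan picks the closest hostile, falling back to enemy capital ships, and leads its position by velocity.
; A gated Tick rotates toward the target and thrusts forward.
; A timed front trace triggers avoidance along a random unblocked direction; a separate sequence handles hangar launches.
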(event `CheckForTargets`
  (bind _primarytarget (`self.PrimaryTarget`))
  (bind _controlledship (`self.ControlledShip`))
  (bind _returnvalue (`self.K2_GetActorLocation` _controlledship))
  ;[1 1 1] Performs a sphere trace around the actor searching for targets that implement "Interface_TargetableByTurrets"
  (bind _outhits (`KismetSystemLibrary.SphereTraceMultiForObjects` _returnvalue (+ _returnvalue (0.0 0.0 10.0)) 4000.0 (`|MakeArray` "ObjectTypeQuery3" :!type "EObjectTypeQuery Enum") false (`|MakeArray` _controlledship :!type "Actor Object Reference")))
  (for _array_element _outhits
    (bind (_bblockinghit _binitialoverlap _time _location _impactpoint _normal _impactnormal _physmat _hitactor) (`GameplayStatics.BreakHitResult` _array_element))
    (if (`KismetSystemLibrary.DoesImplementInterface` _hitactor "/Game/SpaceCombatKit/Blueprints/Turrets/Interfaces/Interf_TurretTarget.Interf_TurretTarget_C")
      (bind _asbase_ship (cast `/Game/SpaceCombatKit/Blueprints/Ships/BaseClasses/BaseShip` _hitactor))
      (if (`|EnumInequality` (`/Game/SpaceCombatKit/Blueprints/Ships/BaseClasses/BaseShip.Faction` _asbase_ship) (`/Game/SpaceCombatKit/Blueprints/Ships/BaseClasses/BaseShip.Faction` (`self.ControlledShip`)))
        (`KismetArrayLibrary.Array_AddUnique` (`self.Targets`) _hitactor))))
  ;[1 1 1] Gets the shortest distance target, sets it as primary, and gets it's location + velocity to set as target locaiton
  (`self.SortDistanceToTargets`)
  (`/Engine/EditorBlueprintResources/StandardMacros.IsValid` _primarytarget
    (:`Is Valid`
      (set `self.TargetLocation` (+ (`self.K2_GetActorLocation` _primarytarget) (`self.GetVelocity` _primarytarget)))
      (`self.OpenTick`))
    (:`Is Not Valid`
      ;[1 1 1] Get a capital ship target if they exist
      (if (`KismetArrayLibrary.Array_IsValidIndex` (`/Game/SpaceCombatKit/Blueprints/Ships/BaseClasses/BaseShip.EnemyCapitals` (`self.ControlledShip`)))
        (`self.GetCapitalTargetAndFlyToIt`)))))

(event `self.ReceiveBeginPlay`
  ;[1 1 1] on possess, get controlled pawn and cast it to baseship. Set that as ControlledShip.
)

(event `self.OnPossess`
  (params (PossessedPawn :type "Pawn Object Reference"))
  ;[1 1 1] on possess, get controlled pawn and cast it to baseship. Set that as ControlledShip.
  (bind _asbase_ship (cast `/Game/SpaceCombatKit/Blueprints/Ships/BaseClasses/BaseShip` PossessedPawn))
  (bind _output_get (set `self.ControlledShip` _asbase_ship))
  (if (`self.DestroyPawnCockpit`)
    (`/Game/SpaceCombatKit/Blueprints/Ships/BaseClasses/BaseShip.DestroyCockpit` _output_get))
  (if (`self.StartsLaunched`)
    ;[1 1 1] check if we have patrol points, if so, set patrolling, and fly to the first one
    (if (> (`KismetArrayLibrary.Array_LastIndex` (`/Game/SpaceCombatKit/Blueprints/Ships/BaseClasses/BaseShip.PatrolPoints` (`self.ControlledShip`))) 0) :!label _label
      (set `self.Patrolling` true)
      (`self.FlyToNextPatrolPoint`))
    (`KismetSystemLibrary.K2_SetTimerDelegate` (delegate `CheckForTargets`) (`self.EnemyDetectionPulse`) true)
    (`KismetSystemLibrary.K2_SetTimerDelegate` (delegate `CheckFront`) (`self.CollisionPulse`) true)))

(event `LaunchFromhangar`
  (bind _controlledship (`self.ControlledShip`))
  ;[1 1 1] Launch from hangar - after a few seconds, open the gate to move forward, then after that open tick gate and close this gate to complete the launch sequence
  (`KismetSystemLibrary.Delay` 2.0)
  (goto _label_3 :!via `Open`))

(event `CheckFront`
  ;[1 1 1] Check front pulse. If there's a hit, get an available strafing direction. Reset direction after 2 sec
  (bind _overlap (`self.CheckForFrontCollision` (`self.CollisionTraceDistance`)))
  (bind _output_get (set `self.FrontOverlap` _overlap))
  (if _output_get
    (`/Engine/EditorBlueprintResources/StandardMacros.DoOnce` false :!label _label_2
      (:`Completed`
        (`self.SetFlightDirectionsCheckingCollisions`)
        (`KismetSystemLibrary.Delay` 2.0)
        (goto _label_2 :!via `Reset`)))))

(event `self.ReceiveTick`
  (params (DeltaSeconds :type "Float (single-precision)"))
  (bind _primarytarget (`self.PrimaryTarget`))
  (bind _controlledship (`self.ControlledShip`))
  (bind _primarytarget_2 (`self.PrimaryTarget`))
  (bind _controlledship_2 (`self.ControlledShip`))
  (bind _returnvalue (`self.K2_GetActorLocation` _primarytarget))
  (`|ExecutionSequence`
    (:`then_0`
      ;[1 1 1] Launch from hangar - after a few seconds, open the gate to move forward, then after that open tick gate and close this gate to complete the launch sequence
      (`/Engine/EditorBlueprintResources/StandardMacros.Gate` (`self.StartsLaunched`) :!label _label_3
        (:`Exit`
          (`Pawn.AddMovementInput` _controlledship (`self.GetActorForwardVector` _controlledship) 1.0 false)
          (`KismetSystemLibrary.Delay` 2.25)
          (`self.OpenTick`)
          (`|ExecutionSequence`
            (:`then_0`
              (goto _label_3 :!via `Close`))
            (:`then_1`
              (goto _label))))))
    (:`then_1`
      ;[1 1 1] If the gate has been opened (fly order issued), chck if there's a target location
      (`/Engine/EditorBlueprintResources/StandardMacros.Gate` true :!label _label_4
        (:`Exit`
          (if (!= (`self.TargetLocation`) (0.0 0.0 0.0))
            ;[1 1 1] Checks distance to target
            (`|ExecutionSequence`
              (:`then_0`
                (if (> (`self.CheckDistanceToTarget`) (`self.MoveToAcceptanceDistance`))
                  ;[1 1 1] If there's a front collision, engage avoidance. Otherwise fly straight
                  (if (`self.FrontOverlap`)
                    ;[1 1 1] There was a front collision, so fly in a direction chosen by Set Flight Directions Checking Collisions
                    (`Pawn.AddMovementInput` _controlledship_2 (`KismetArrayLibrary.Array_Get` (`self.FlightDirections`) (`self.FlightDirectionChoiceIndex`)) 1.0 false)
                    (`/Engine/EditorBlueprintResources/StandardMacros.IsValid` (`self.PrimaryTarget`)
                      (:`Is Valid`
                        (`self.RotateToFaceTargetLocation` (+ (`self.K2_GetActorLocation` _primarytarget_2) (* (`self.GetVelocity` _primarytarget_2) 0.75))))
                      (:`Is Not Valid`
                        (`self.RotateToFaceTargetLocation` (`self.TargetLocation`))))
                    (else
                      ;[1 1 1] If nothing in front of pawn, rotate to face target location. If facing it within Error Tolerance, add forward input
                      (`self.RotateToFaceTargetLocation` (`self.TargetLocation`))
                      (if (`self.CheckIfFacingTarget`)
                        (`Pawn.AddMovementInput` _controlledship_2 (`self.GetActorForwardVector` _controlledship_2) 1.0 false))))
                  (else
                    ;[1 1 1] If we have a valid enemy target, face it, and interping it's velocity
                    (`/Engine/EditorBlueprintResources/StandardMacros.IsValid` _primarytarget
                      (:`Is Valid`
                        (`self.RotateToFaceTargetLocation` (`KismetMathLibrary.VInterpTo` _returnvalue (+ _returnvalue (`self.GetVelocity` _primarytarget)) (`GameplayStatics.GetWorldDeltaSeconds`) 6.0)))
                      (:`Is Not Valid`
                        ;[1 1 1] If we're within range of target location, check if we patrol. If so, delay, then get next point. If not, clear target locationto go idle
                        (if (`self.Patrolling`)
                          (`KismetSystemLibrary.Delay` 5.0)
                          (`self.FlyToNextPatrolPoint`)
                          (else
                            (set `self.TargetLocation` (0.0 0.0 0.0))
                            (`self.CloseTick`))))))))
              (:`then_1`
                ;[1 1 1] If we have a target and we're within range, open fire
                (`/Engine/EditorBlueprintResources/StandardMacros.IsValid` (`self.PrimaryTarget`)
                  (:`Is Valid`
                    (for _array_element (`/Game/SpaceCombatKit/Blueprints/Ships/BaseClasses/BaseShip.PrimaryWeapons` (`self.ControlledShip`))
                      (set `/Game/SpaceCombatKit/Blueprints/Weapons/BaseWeapon.WantsToFire` (not (> (`self.CheckDistanceToTarget`) (* (`self.MoveToAcceptanceDistance`) 1.75))) _array_element)))
                  (:`Is Not Valid`
                    (for _array_element_2 (`/Game/SpaceCombatKit/Blueprints/Ships/BaseClasses/BaseShip.PrimaryWeapons` (`self.ControlledShip`))
                      (set `/Game/SpaceCombatKit/Blueprints/Weapons/BaseWeapon.WantsToFire` false _array_element_2))
                    (set `self.PrimaryTarget` null)))))
            (else
              (goto _label_4 :!via `Close`))))))))

(event `OpenTick`
  ;[1 1 1] If the gate has been opened (fly order issued), chck if there's a target location
  (goto _label_4 :!via `Open`))

(event `CloseTick`
  ;[1 1 1] If the gate has been opened (fly order issued), chck if there's a target location
  (goto _label_4 :!via `Close`))

(fn `CheckDistanceToTarget`
  (returns (Distance :type "Float (double-precision)"))
  (return (`KismetMathLibrary.VSize` (- (`self.K2_GetActorLocation` (`self.ControlledShip`)) (`self.TargetLocation`)))))

(fn `CheckForCollisionAtDirection`
  (params (Distance :type "Float (double-precision)") (TraceDirection :type "Vector Structure"))
  (returns (Overlap :type Boolean))
  (bind _controlledship (`self.ControlledShip`))
  (bind _returnvalue (`self.K2_GetActorLocation` _controlledship))
  ;[1 1 1] Runs a lsphere trace the size of the controlled ship along the given direction with a length of the given distance, to detect if there's something in the way
  (bind (_outhit _returnvalue_2) (`KismetSystemLibrary.SphereTraceSingle` _returnvalue (+ _returnvalue (* TraceDirection Distance)) (* (`CapsuleComponent.GetUnscaledCapsuleRadius` (`Character.CapsuleComponent` _controlledship)) 3.0) "TraceTypeQuery1" false (`|MakeArray` _controlledship :!type "Actor Object Reference")))
  (return _returnvalue_2))

(fn `CheckForFrontCollision`
  (params (Distance :type "Float (double-precision)"))
  (returns (Overlap :type Boolean))
  (bind _controlledship (`self.ControlledShip`))
  (bind _returnvalue (`self.K2_GetActorLocation` _controlledship))
  (bind (_outhit _returnvalue_2) (`KismetSystemLibrary.SphereTraceSingle` _returnvalue (+ _returnvalue (* (+ (`self.GetActorForwardVector` _controlledship) (`KismetMathLibrary.Normal` (`self.GetVelocity` _controlledship))) Distance)) (* (`CapsuleComponent.GetUnscaledCapsuleRadius` (`Character.CapsuleComponent` _controlledship)) 3.0) "TraceTypeQuery2" false (`|MakeArray` _controlledship :!type "Actor Object Reference")))
  (return _returnvalue_2))

(fn `CheckIfFacingTarget`
  (returns (NewParam :type Boolean))
  (bind _returnvalue (`self.K2_GetPawn`))
  ;[1 1 1] Checks if our pawn is facing our target within error tolerance and returns true or false
  (if (== (`self.K2_GetActorRotation` _returnvalue) (`KismetMathLibrary.FindLookAtRotation` (`self.K2_GetActorLocation` _returnvalue) (`self.TargetLocation`)) :`ErrorTolerance` (`self.LookAtMovementErrorTolerance`))
    (return true)
    (else
      (return false))))

(fn `FlyToLocation`
  (params (TargetLocation :type "Vector Structure"))
  ;[1 1 1] Sets the target location, and opens tick so we can start flying
  (set `self.TargetLocation` TargetLocation)
  (`self.OpenTick`))

(fn `FlyToNextPatrolPoint`
  (bind _currentpatrolpointindex (`self.CurrentPatrolPointIndex`))
  (bind _returnvalue (+ _currentpatrolpointindex 1))
  (bind _patrolpoints (`/Game/SpaceCombatKit/Blueprints/Ships/BaseClasses/BaseShip.PatrolPoints` (`self.ControlledShip`)))
  ;[1 1 1] Flies to the current patrol point, then checks if the next patrol point is valid. If it's not, restart by setting index to 0
  (`self.FlyToLocation` (`self.K2_GetActorLocation` (`KismetArrayLibrary.Array_Get` _patrolpoints _currentpatrolpointindex)))
  (if (`KismetArrayLibrary.Array_IsValidIndex` _patrolpoints _returnvalue)
    (set `self.CurrentPatrolPointIndex` _returnvalue)
    (else
      (set `self.CurrentPatrolPointIndex` 0))))

(fn `GetCapitalTargetAndFlyToIt`
  (bind _primarytarget (`self.PrimaryTarget`))
  ;[1 1 1] Get's the controlled ships list of enemy capitals, and sets it as targets. Then tells it to sort them, and fly to the main (closest) target.
  (set `self.Targets` (`/Game/SpaceCombatKit/Blueprints/Ships/BaseClasses/BaseShip.EnemyCapitals` (`self.ControlledShip`)))
  (`self.SortDistanceToTargets`)
  (`/Engine/EditorBlueprintResources/StandardMacros.IsValid` _primarytarget
    (:`Is Valid`
      (`self.FlyToLocation` (`self.K2_GetActorLocation` _primarytarget)))))

(fn `RotateToFaceTargetLocation`
  (params (Target :type "Vector Structure (by ref)"))
  (bind _controlledship (`self.ControlledShip`))
  (bind _returnvalue (`KismetMathLibrary.VSize` (`self.GetVelocity` _controlledship)))
  ;[1 1 1] Finds the look at rotation to given vector, adding our velocity * our speed to it
  (`self.K2_SetActorRotation` (`self.ControlledShip`) (`KismetMathLibrary.RInterpTo` (`self.K2_GetActorRotation` _controlledship) (`KismetMathLibrary.FindLookAtRotation` (+ (`self.K2_GetActorLocation` _controlledship) (* (`self.GetVelocity` _controlledship) (`KismetMathLibrary.MapRangeClamped` _returnvalue 0.0 2000.0 0.3 1.0))) Target) (`GameplayStatics.GetWorldDeltaSeconds`) (* (`KismetMathLibrary.MapRangeClamped` _returnvalue 0.0 2000.0 -2.0 -1.0) -1.0)) false))

(fn `SetFlightDirectionsCheckingCollisions`
  (locals (Timer :type Integer))
  (bind _controlledship (`self.ControlledShip`))
  (bind _returnvalue (`self.GetActorUpVector` _controlledship))
  (bind _returnvalue_2 (`self.GetActorRightVector` _controlledship))
  (bind _returnvalue_3 (`self.GetActorForwardVector` _controlledship))
  (bind _returnvalue_4 (* _returnvalue_2 -1.0))
  (bind _returnvalue_5 (* _returnvalue -1.0))
  (bind _returnvalue_6 (+ _returnvalue _returnvalue_2))
  (bind _returnvalue_7 (+ _returnvalue_5 _returnvalue_4))
  ;[1 1 1] Set flight directions based on forward vector
  (bind _output_get (set `self.FlightDirections` (`|MakeArray` (+ _returnvalue _returnvalue_3) (+ _returnvalue_5 _returnvalue_3) (+ _returnvalue_6 _returnvalue_3) (+ _returnvalue_2 _returnvalue_3) (+ _returnvalue_4 _returnvalue_3) (+ (* _returnvalue_6 -1.0) _returnvalue_3) (+ _returnvalue_7 _returnvalue_3) (+ (* _returnvalue_7 -1.0) _returnvalue_3))))
  ;[1 1 1] Checks all directions for overlaps to determine if we can actually move that way. If we can't, remove it
  (for _array_element _output_get
    (bind _overlap (`self.CheckForCollisionAtDirection` (`self.CollisionTraceDistance`) _array_element))
    (if _overlap
      (`KismetArrayLibrary.Array_RemoveItem` (`self.FlightDirections`) _array_element)))
  ;[1 1 1] Get a random direction from the available directions
  (if (`KismetArrayLibrary.Array_IsValidIndex` _output_get)
    (set `self.FlightDirectionChoiceIndex` (`KismetMathLibrary.RandomIntegerInRange` 0 (`KismetArrayLibrary.Array_LastIndex` _output_get)))
    (else
      ;[1 1 1] If there are no directions we can move.. move backwards
      (set `self.FlightDirections` (`|MakeArray` (* (`self.GetActorForwardVector` (`self.ControlledShip`)) -1.0))))))

(fn `SortDistanceToTargets`
  (locals (ClosestDistanceCheck :type "Float (double-precision)") (TempPrimaryTarget :type "Actor Object Reference"))
  ;[1 1 1] Clears the local variables so the data will be fresh
  (set `local.ClosestDistanceCheck` 50000.0)
  (set `local.TempPrimaryTarget` null)
  ;[1 1 1] For each target, checks if we can see it. If we can, checks if it's closer than the last target we could see. If it is, set it to the temporary primary target
  (for _array_element (`self.Targets`)
    (`/Engine/EditorBlueprintResources/StandardMacros.IsValid` _array_element
      (:`Is Valid`
        (bind _returnvalue (`self.GetDistanceTo` (`self.ControlledShip`) _array_element))
        (if (< _returnvalue (`local.ClosestDistanceCheck`))
          (set `local.ClosestDistanceCheck` _returnvalue)
          (set `local.TempPrimaryTarget` _array_element)))))
  ;[1 1 1] Sets the primary target to the temporary primary target
  (`/Engine/EditorBlueprintResources/StandardMacros.IsValid` (`local.TempPrimaryTarget`)
    (:`Is Valid`
      (set `self.PrimaryTarget` (`local.TempPrimaryTarget`)))))

(fn `UserConstructionScript`)