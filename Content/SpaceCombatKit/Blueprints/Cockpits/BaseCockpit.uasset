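; Base cockpit actor for a player ship, spawned as its child actor, with health displays and joystick animation.
; BeginPlay caches the parent ship, sets it as owner for owner-only visibility, and calls an empty VR touch hook when HMD and motion controllers are present.
; SetUpWidgets links health widgets to the ship and its capitals, removing those without targets.
; CalculateJoystickRotation eases a stick toward the ship's local-space movement input.
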(event `self.ReceiveBeginPlay`
  (bind _returnvalue (`self.GetParentActor`))
  ;[1 1 1] Begin play - set parent ship and set up widgets. Then set owner for Owner Only See Visibility
  (bind _asbase_ship (cast `/Game/SpaceCombatKit/Blueprints/Ships/BaseClasses/BaseShip` _returnvalue))
  (set `self.ParentShip` _asbase_ship)
  (`self.SetOwner` _returnvalue)
  ;[1 1 1] Sets up VR interaction with the cockpit if both touch is enabled and the HMD is enabled
  (if (and (`HeadMountedDisplayFunctionLibrary.IsHeadMountedDisplayEnabled`) (> (`MotionTrackedDeviceFunctionLibrary.GetMotionTrackingEnabledControllerCount`) 0))
    (`self.SetUpVRTouchInteraction`)))

(fn `AddEnemyCapitalWidgets`
  (bind _enemycaphealth (`self.EnemyCapHealth`))
  ;[1 1 1] Clears children in the array so we don't get duplicates
  (bind _asumg_ship_health_array (cast `/Game/SpaceCombatKit/UMGWidgets/UMG_ShipHealthArray` (`WidgetComponent.GetUserWidgetObject` _enemycaphealth)))
  (bind _verticalboxhealtharray (`/Game/SpaceCombatKit/UMGWidgets/UMG_ShipHealthArray.VerticalBoxHealthArray` _asumg_ship_health_array))
  (`PanelWidget.ClearChildren` _verticalboxhealtharray)
  ;[1 1 1] Gets the ship that owns this cockpit / display
  (bind _asbase_ship (cast `/Game/SpaceCombatKit/Blueprints/Ships/BaseClasses/BaseShip` (`self.GetParentActor`)))
  (bind _enemycapitals (`/Game/SpaceCombatKit/Blueprints/Ships/BaseClasses/BaseShip.EnemyCapitals` _asbase_ship))
  ;[1 1 1] If there are no enemy capitals delete the health array component
  (`/Engine/EditorBlueprintResources/StandardMacros.IsValid` (`|GetArrayItem` _enemycapitals)
    (:`Is Valid`
      ;[1 1 1] For each enemy capital create a ship health widget and add it to the array
      (for _array_element _enemycapitals
        (bind _returnvalue (`|CreateWidget` "/Game/SpaceCombatKit/UMGWidgets/UMG_ShipHealthWidget.UMG_ShipHealthWidget_C" (cast `PlayerController` (`Pawn.GetController` (cast `Pawn` (`self.GetParentActor`) :!pure true)) :!pure true)))
        (`PanelWidget.AddChild` _verticalboxhealtharray _returnvalue)
        (set `/Game/SpaceCombatKit/UMGWidgets/UMG_ShipHealthWidget.Ship` _array_element _returnvalue)
        (set `/Game/SpaceCombatKit/UMGWidgets/UMG_ShipHealthWidget.TextBind` "Enemy Capital" _returnvalue)))
    (:`Is Not Valid`
      (`ActorComponent.K2_DestroyComponent` _enemycaphealth))))

(fn `CalculateJoystickRotation`
  (params (Joystick :type "SceneComponent Object Reference"))
  (returns (DesiredRotation :type "Rotator Structure"))
  (bind _parentship (`self.ParentShip`))
  (bind (_returnvalue_x _returnvalue_y) (`KismetMathLibrary.BreakVector` (`KismetMathLibrary.InverseTransformDirection` (`self.GetTransform` _parentship) (`PawnMovementComponent.GetLastInputVector` (`Character.CharacterMovement` _parentship)))))
  (return (`KismetMathLibrary.RInterpTo` (`SceneComponent.RelativeRotation` Joystick) (`KismetMathLibrary.MakeRotator` 0.0 (* (`KismetMathLibrary.MapRangeClamped` _returnvalue_x -1.0 1.0 -20.0 20.0) -1.0) (* (`KismetMathLibrary.MapRangeClamped` _returnvalue_y -1.0 1.0 -20.0 20.0) -1.0)) (`GameplayStatics.GetWorldDeltaSeconds`) (`self.JoystickInterpSpeed`))))

(fn `SetUpVRTouchInteraction`)

(fn `SetUpWidgets`
  (bind _friendlycaphealth (`self.FriendlyCapHealth`))
  (bind _asumg_ship_health_widget (cast `/Game/SpaceCombatKit/UMGWidgets/UMG_ShipHealthWidget` (`WidgetComponent.GetUserWidgetObject` (`self.SelfHealth`)) :!pure true))
  (bind _asumg_ship_health_widget_2 (cast `/Game/SpaceCombatKit/UMGWidgets/UMG_ShipHealthWidget` (`WidgetComponent.GetUserWidgetObject` _friendlycaphealth) :!pure true))
  ;[1 1 1] Checks if friendly/enemy capitals are valid. If not, destroy Capital health widgets. If they are valid, link their health
  (bind _asbase_ship (cast `/Game/SpaceCombatKit/Blueprints/Ships/BaseClasses/BaseShip` (`self.GetParentActor`)))
  (bind _output (`|GetArrayItem` (`/Game/SpaceCombatKit/Blueprints/Ships/BaseClasses/BaseShip.FriendlyCapitals` _asbase_ship)))
  (`/Engine/EditorBlueprintResources/StandardMacros.IsValid` _output
    (:`Is Valid`
      (set `/Game/SpaceCombatKit/UMGWidgets/UMG_ShipHealthWidget.Ship` _output _asumg_ship_health_widget_2)
      (set `/Game/SpaceCombatKit/UMGWidgets/UMG_ShipHealthWidget.TextBind` "Friendly Capital" _asumg_ship_health_widget_2))
    (:`Is Not Valid`
      (`ActorComponent.K2_DestroyComponent` _friendlycaphealth)))
  (`self.AddEnemyCapitalWidgets`)
  ;[1 1 1] Self Health Widget
  (set `/Game/SpaceCombatKit/UMGWidgets/UMG_ShipHealthWidget.Ship` (cast `/Game/SpaceCombatKit/Blueprints/Ships/BaseClasses/BaseShip` (`self.GetParentActor`) :!pure true) _asumg_ship_health_widget)
  (set `/Game/SpaceCombatKit/UMGWidgets/UMG_ShipHealthWidget.TextBind` "Health" _asumg_ship_health_widget))

(fn `UserConstructionScript`)