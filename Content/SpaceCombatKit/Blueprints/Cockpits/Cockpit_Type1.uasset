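; Cockpit Blueprint for a space combat ship, with a child-actor weapons panel that displays the ship's weapon information.
; On BeginPlay it passes the parent ship to the panel's weapons display widget as the owning ship and refreshes the widget's variables.
; It also sets the widget's owning player from the ship's controller and makes the ship the panel's owner.
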(event `self.ReceiveBeginPlay`
  (bind _asbase_ship (cast `/Game/SpaceCombatKit/Blueprints/Ships/BaseClasses/BaseShip` (`self.GetParentActor`) :!pure true))
  (bind _ascockpit_panel_weapons (cast `/Game/SpaceCombatKit/Blueprints/Cockpits/CockpitPanel_Weapons` (`ChildActorComponent.ChildActor` (`self.WeaponsPanel`)) :!pure true))
  (bind _asumg_weapons_display (cast `/Game/SpaceCombatKit/UMGWidgets/UMG_WeaponsDisplay` (`WidgetComponent.GetUserWidgetObject` (`/Game/SpaceCombatKit/Blueprints/Cockpits/CockpitPanel_Weapons.Widget` _ascockpit_panel_weapons)) :!pure true))
  ;[1 1 1] Begin play, tell the weapons panel who the ship that owns us is so it can get weapons info
  (`parent.ReceiveBeginPlay`)
  (set `/Game/SpaceCombatKit/UMGWidgets/UMG_WeaponsDisplay.OwningShip` _asbase_ship _asumg_weapons_display)
  (`/Game/SpaceCombatKit/UMGWidgets/UMG_WeaponsDisplay.UpdateVariables` _asumg_weapons_display)
  (`UserWidget.SetOwningPlayer` _asumg_weapons_display (cast `PlayerController` (`Pawn.GetController` _asbase_ship) :!pure true))
  (`self.SetOwner` _ascockpit_panel_weapons _asbase_ship))

(fn `UserConstructionScript`
  (`parent.UserConstructionScript`))